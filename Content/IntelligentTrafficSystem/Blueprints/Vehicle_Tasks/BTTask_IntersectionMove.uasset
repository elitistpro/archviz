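; Behavior tree task that drives an AI traffic car through an intersection at low speed in the Intelligent Traffic System.
; If the speed limiter stop flag is set, it cuts throttle and brakes; otherwise it refreshes the car's path and forces first gear.
; It then brakes when speed in km/h exceeds the car's MaxSpeed, or else lowers that limit to a fixed value and applies moderate throttle.
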(event EventReceiveExecuteAI
  (params (OwnerController :type AI%20Controller%20Object%20Reference) (ControlledPawn :type Pawn%20Object%20Reference))
  (bind _asbp_ai_car (Utilities|Casting|CastToBP_Ai_car ControlledPawn))
  (if (Variables|/Game/IntelligentTrafficSystem/Blueprints/Vehicle_BPs/BP_Ai_car.BP_Ai_car_C|GetStop%20for%20speed%20limiter _asbp_ai_car)
    (Class|ChaosVehicleMovementComponent|SetThrottleInput (Variables|/Script/ChaosVehicles.WheeledVehiclePawn|GetVehicleMovementComponent _asbp_ai_car) 0.0 :!label _label)
    (Class|ChaosVehicleMovementComponent|SetBrakeInput (Variables|/Script/ChaosVehicles.WheeledVehiclePawn|GetVehicleMovementComponent _asbp_ai_car) 0.5)
    (Class|ChaosVehicleMovementComponent|SetHandbrakeInput (Variables|/Script/ChaosVehicles.WheeledVehiclePawn|GetVehicleMovementComponent _asbp_ai_car) false)
    (AI|BehaviorTree|FinishExecute true)
    (else
      (Default|GetPath _asbp_ai_car)
      (Class|ChaosVehicleMovementComponent|SetTargetGear (Variables|/Script/ChaosVehicles.WheeledVehiclePawn|GetVehicleMovementComponent _asbp_ai_car) 1 true)
      (if (> (* (Class|ChaosVehicleMovementComponent|GetForwardSpeedMPH (Variables|/Script/ChaosVehicles.WheeledVehiclePawn|GetVehicleMovementComponent _asbp_ai_car)) 1.609) (Variables|/Game/IntelligentTrafficSystem/Blueprints/Vehicle_BPs/BP_Ai_car.BP_Ai_car_C|GetMax%20Speed _asbp_ai_car))
        (goto _label)
        (else
          (Variables|/Game/IntelligentTrafficSystem/Blueprints/Vehicle_BPs/BP_Ai_car.BP_Ai_car_C|SetMax%20Speed _asbp_ai_car 2e+01)
          (Class|ChaosVehicleMovementComponent|SetThrottleInput (Variables|/Script/ChaosVehicles.WheeledVehiclePawn|GetVehicleMovementComponent _asbp_ai_car) 0.5)
          (Class|ChaosVehicleMovementComponent|SetBrakeInput (Variables|/Script/ChaosVehicles.WheeledVehiclePawn|GetVehicleMovementComponent _asbp_ai_car) 0.0)
          (Class|ChaosVehicleMovementComponent|SetHandbrakeInput (Variables|/Script/ChaosVehicles.WheeledVehiclePawn|GetVehicleMovementComponent _asbp_ai_car) false)
          (AI|BehaviorTree|FinishExecute true))))))