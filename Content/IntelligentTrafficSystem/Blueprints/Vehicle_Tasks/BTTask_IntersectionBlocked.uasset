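; Behavior tree task that decides whether an AI traffic car waits or drives on at a blocked intersection.
; After refreshing its path, it compares intersection timestamps with the obstructing car, randomly bumping its own on a tie.
; It throttles forward only with the higher timestamp and a nearly stopped obstructor, otherwise braking with rear lights on.
; Without a valid obstructor it clears the IntersectionBlocked blackboard key and drives on.
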(event EventReceiveExecuteAI
  (params (OwnerController :type AI%20Controller%20Object%20Reference) (ControlledPawn :type Pawn%20Object%20Reference))
  (bind _asbp_ai_car (Utilities|Casting|CastToBP_Ai_car ControlledPawn))
  (Default|GetPath _asbp_ai_car)
  (Utilities|IsValid (Variables|/Game/IntelligentTrafficSystem/Blueprints/Vehicle_BPs/BP_Ai_car.BP_Ai_car_C|GetIntersection%20obstructing%20car _asbp_ai_car)
    (:Is%20Valid
      (if (== (Variables|/Game/IntelligentTrafficSystem/Blueprints/Vehicle_BPs/BP_Ai_car.BP_Ai_car_C|GetIntersection%20timestamp _asbp_ai_car) (Variables|/Game/IntelligentTrafficSystem/Blueprints/Vehicle_BPs/BP_Ai_car.BP_Ai_car_C|GetIntersection%20timestamp (Variables|/Game/IntelligentTrafficSystem/Blueprints/Vehicle_BPs/BP_Ai_car.BP_Ai_car_C|GetIntersection%20obstructing%20car _asbp_ai_car)))
        (Variables|/Game/IntelligentTrafficSystem/Blueprints/Vehicle_BPs/BP_Ai_car.BP_Ai_car_C|SetIntersection%20timestamp _asbp_ai_car (+ (Variables|/Game/IntelligentTrafficSystem/Blueprints/Vehicle_BPs/BP_Ai_car.BP_Ai_car_C|GetIntersection%20timestamp _asbp_ai_car) (Math|Random|RandomIntegerinRange 1 5))))
      (if (> (Variables|/Game/IntelligentTrafficSystem/Blueprints/Vehicle_BPs/BP_Ai_car.BP_Ai_car_C|GetIntersection%20timestamp _asbp_ai_car) (Variables|/Game/IntelligentTrafficSystem/Blueprints/Vehicle_BPs/BP_Ai_car.BP_Ai_car_C|GetIntersection%20timestamp (Variables|/Game/IntelligentTrafficSystem/Blueprints/Vehicle_BPs/BP_Ai_car.BP_Ai_car_C|GetIntersection%20obstructing%20car _asbp_ai_car)))
        (if (> (Variables|/Game/IntelligentTrafficSystem/Blueprints/Vehicle_BPs/BP_Ai_car.BP_Ai_car_C|GetCurrent%20speed (Variables|/Game/IntelligentTrafficSystem/Blueprints/Vehicle_BPs/BP_Ai_car.BP_Ai_car_C|GetIntersection%20obstructing%20car _asbp_ai_car)) 5.0)
          (Default|RearLights _asbp_ai_car 1.0 :!label _label)
          (Class|ChaosVehicleMovementComponent|SetBrakeInput (Variables|/Script/ChaosVehicles.WheeledVehiclePawn|GetVehicleMovementComponent _asbp_ai_car) 1.0)
          (AI|BehaviorTree|FinishExecute true)
          (else
            (Class|ChaosVehicleMovementComponent|SetBrakeInput (Variables|/Script/ChaosVehicles.WheeledVehiclePawn|GetVehicleMovementComponent _asbp_ai_car) 0.0 :!label _label_2)
            (Default|RearLights _asbp_ai_car 0.0)
            (Class|ChaosVehicleMovementComponent|SetThrottleInput (Variables|/Script/ChaosVehicles.WheeledVehiclePawn|GetVehicleMovementComponent _asbp_ai_car) 0.5)
            (AI|BehaviorTree|FinishExecute true)))
        (else
          (goto _label))))
    (:Is%20Not%20Valid
      (Class|BTFunctionLibrary|SetBlackboardValueasBool (Variables|Default|GetIntersection%20blocked) false)
      (goto _label_2))))