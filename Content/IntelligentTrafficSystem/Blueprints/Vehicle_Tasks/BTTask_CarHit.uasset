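; Behavior tree task for AI traffic cars that resolves a CarHit blockage at intersections.
; When the car is blocked left or right, it reads the Stop key from the obstructing car's blackboard.
; If that car is stopped, this car brakes on a shared path, otherwise clears CarHit and drives forward in first gear.
; If it is not stopped, this car reverses at light throttle; each branch finishes immediately as successful.
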(event EventReceiveExecuteAI
  (params (OwnerController :type AI%20Controller%20Object%20Reference) (ControlledPawn :type Pawn%20Object%20Reference))
  (bind _asbp_ai_car (Utilities|Casting|CastToBP_Ai_car ControlledPawn))
  (Variables|Default|SetAs%20BP%20Ai%20Car _asbp_ai_car)
  (if (or (Variables|/Game/IntelligentTrafficSystem/Blueprints/Vehicle_BPs/BP_Ai_car.BP_Ai_car_C|GetIntersection%20Left%20Blocked _asbp_ai_car) (Variables|/Game/IntelligentTrafficSystem/Blueprints/Vehicle_BPs/BP_Ai_car.BP_Ai_car_C|GetIntersection%20Right%20Blocked _asbp_ai_car))
    (if (ScalableFloat|GetValueasBool (AI|GetBlackboard (Variables|/Game/IntelligentTrafficSystem/Blueprints/Vehicle_BPs/BP_Ai_car.BP_Ai_car_C|GetIntersection%20obstructing%20car _asbp_ai_car)) (Utilities|Name|MakeLiteralName "Stop"))
      (if (Utilities|Enum|Equal(Enum) (Variables|/Game/IntelligentTrafficSystem/Blueprints/Vehicle_BPs/BP_Ai_car.BP_Ai_car_C|GetActive%20Path%20name _asbp_ai_car) (Variables|/Game/IntelligentTrafficSystem/Blueprints/Vehicle_BPs/BP_Ai_car.BP_Ai_car_C|GetActive%20Path%20name (Variables|/Game/IntelligentTrafficSystem/Blueprints/Vehicle_BPs/BP_Ai_car.BP_Ai_car_C|GetIntersection%20obstructing%20car _asbp_ai_car)))
        (Class|ChaosVehicleMovementComponent|SetBrakeInput (Variables|/Script/ChaosVehicles.WheeledVehiclePawn|GetVehicleMovementComponent _asbp_ai_car) 1.0)
        (AI|BehaviorTree|FinishExecute true :!label _label)
        (else
          (Class|ChaosVehicleMovementComponent|SetBrakeInput (Variables|/Script/ChaosVehicles.WheeledVehiclePawn|GetVehicleMovementComponent _asbp_ai_car) 0.0)
          (Class|BTFunctionLibrary|SetBlackboardValueasBool (Variables|Default|GetCar%20Hit) false)
          (Class|ChaosVehicleMovementComponent|SetTargetGear (Variables|/Script/ChaosVehicles.WheeledVehiclePawn|GetVehicleMovementComponent _asbp_ai_car) 1 true)
          (Class|ChaosVehicleMovementComponent|SetThrottleInput (Variables|/Script/ChaosVehicles.WheeledVehiclePawn|GetVehicleMovementComponent _asbp_ai_car) 0.3)
          (AI|BehaviorTree|FinishExecute true)))
      (else
        (Class|ChaosVehicleMovementComponent|SetTargetGear (Variables|/Script/ChaosVehicles.WheeledVehiclePawn|GetVehicleMovementComponent _asbp_ai_car) -1 true)
        (Development|PrintString "Reversing")
        (Class|ChaosVehicleMovementComponent|SetThrottleInput (Variables|/Script/ChaosVehicles.WheeledVehiclePawn|GetVehicleMovementComponent _asbp_ai_car) 0.3)
        (goto _label)))
    (else
      (AI|BehaviorTree|FinishExecute true))))