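; Behavior tree task for traffic-system pedestrians that advances movement along the active spline path and checks whether its end is reached.
; On each execute it calls MoveAlongPath, then measures the pawn's distance to the spline's last point or start, depending on the Forward flag, using a different threshold for each.
; The result sets the pedestrian's ReachedSplineEnd and the SwitchingPaths blackboard bool, and the task always finishes successfully.
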(event EventReceiveExecuteAI
  (params (OwnerController :type AI%20Controller%20Object%20Reference) (ControlledPawn :type Pawn%20Object%20Reference))
  (bind _asbp_pedestrian (Utilities|Casting|CastToBP_Pedestrian ControlledPawn))
  (bind _output_get (Variables|Default|SetAs%20BP%20Pedestrian _asbp_pedestrian))
  (Default|MoveAlongPath _output_get)
  (if (Variables|/Game/IntelligentTrafficSystem/Blueprints/Pedestrian_BPs/BP_Pedestrian.BP_Pedestrian_C|GetForward? (Variables|Default|GetAs%20BP%20Pedestrian))
    (if (< (Math|Vector|Distance(Vector) (Transformation|GetActorLocation (Variables|Default|GetAs%20BP%20Pedestrian)) (Spline|GetLocationatSplinePoint (Variables|/Game/IntelligentTrafficSystem/Blueprints/Pedestrian_BPs/BP_PedestrianPath.BP_PedestrianPath_C|GetSpline (Variables|/Game/IntelligentTrafficSystem/Blueprints/Pedestrian_BPs/BP_Pedestrian.BP_Pedestrian_C|GetActive%20Path (Variables|Default|GetAs%20BP%20Pedestrian))) (Spline|GetNumberOfSplinePoints (Variables|/Game/IntelligentTrafficSystem/Blueprints/Pedestrian_BPs/BP_PedestrianPath.BP_PedestrianPath_C|GetSpline (Variables|/Game/IntelligentTrafficSystem/Blueprints/Pedestrian_BPs/BP_Pedestrian.BP_Pedestrian_C|GetActive%20Path (Variables|Default|GetAs%20BP%20Pedestrian)))) "World")) 5e+01)
      (Development|PrintString "Hello")
      (Variables|/Game/IntelligentTrafficSystem/Blueprints/Pedestrian_BPs/BP_Pedestrian.BP_Pedestrian_C|SetReached%20Spline%20End (Variables|Default|GetAs%20BP%20Pedestrian) true)
      (Class|BTFunctionLibrary|SetBlackboardValueasBool (Variables|Default|GetSwitching%20paths) true)
      (AI|BehaviorTree|FinishExecute true)
      (else
        (Variables|/Game/IntelligentTrafficSystem/Blueprints/Pedestrian_BPs/BP_Pedestrian.BP_Pedestrian_C|SetReached%20Spline%20End (Variables|Default|GetAs%20BP%20Pedestrian) false)
        (Class|BTFunctionLibrary|SetBlackboardValueasBool (Variables|Default|GetSwitching%20paths) false)
        (AI|BehaviorTree|FinishExecute true)))
    (elif (< (Math|Vector|Distance(Vector) (Transformation|GetActorLocation (Variables|Default|GetAs%20BP%20Pedestrian)) (Spline|GetLocationatDistanceAlongSpline (Variables|/Game/IntelligentTrafficSystem/Blueprints/Pedestrian_BPs/BP_PedestrianPath.BP_PedestrianPath_C|GetSpline (Variables|/Game/IntelligentTrafficSystem/Blueprints/Pedestrian_BPs/BP_Pedestrian.BP_Pedestrian_C|GetActive%20Path (Variables|Default|GetAs%20BP%20Pedestrian))) 0.0 "World")) 3e+01)
      (Variables|/Game/IntelligentTrafficSystem/Blueprints/Pedestrian_BPs/BP_Pedestrian.BP_Pedestrian_C|SetReached%20Spline%20End (Variables|Default|GetAs%20BP%20Pedestrian) true)
      (Class|BTFunctionLibrary|SetBlackboardValueasBool (Variables|Default|GetSwitching%20paths) true)
      (AI|BehaviorTree|FinishExecute true)
      (else
        (Variables|/Game/IntelligentTrafficSystem/Blueprints/Pedestrian_BPs/BP_Pedestrian.BP_Pedestrian_C|SetReached%20Spline%20End (Variables|Default|GetAs%20BP%20Pedestrian) false)
        (Class|BTFunctionLibrary|SetBlackboardValueasBool (Variables|Default|GetSwitching%20paths) false)
        (AI|BehaviorTree|FinishExecute true)))))