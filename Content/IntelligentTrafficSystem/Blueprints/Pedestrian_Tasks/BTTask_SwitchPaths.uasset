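; Behavior tree task for Intelligent Traffic System pedestrians that handles the switch to another spline path.
; On looping paths it writes a point near the spline's start or end, depending on direction, to the TargetLocation blackboard key.
; Otherwise it randomly picks a NextPath entry whose relevant endpoint is nearby, then uses AIMoveTo when forward or MoveAlongPath when reversed.
; FinishExecute also fires inside the filtering loops, before the switch.
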(event EventReceiveExecuteAI
  (params (OwnerController :type AI%20Controller%20Object%20Reference) (ControlledPawn :type Pawn%20Object%20Reference))
  (bind _paths_to_switch (Variables|Default|GetPaths%20to%20switch))
  (bind _paths_to_switch_2 (Variables|Default|GetPaths%20to%20switch))
  (bind _asbp_pedestrian (Utilities|Casting|CastToBP_Pedestrian ControlledPawn))
  (bind _output_get (Variables|Default|SetAs%20BP%20Pedestrian _asbp_pedestrian))
  (if (Variables|/Game/IntelligentTrafficSystem/Blueprints/Pedestrian_BPs/BP_PedestrianPath.BP_PedestrianPath_C|GetLoop? (Variables|/Game/IntelligentTrafficSystem/Blueprints/Pedestrian_BPs/BP_Pedestrian.BP_Pedestrian_C|GetActive%20Path _output_get))
    (if (Variables|/Game/IntelligentTrafficSystem/Blueprints/Pedestrian_BPs/BP_Pedestrian.BP_Pedestrian_C|GetForward? (Variables|Default|GetAs%20BP%20Pedestrian))
      (AI|BehaviorTree|SetBlackboardValueasVector (Variables|Default|GetTarget%20location) (Spline|GetLocationatDistanceAlongSpline (Variables|/Game/IntelligentTrafficSystem/Blueprints/Pedestrian_BPs/BP_PedestrianPath.BP_PedestrianPath_C|GetSpline (Variables|/Game/IntelligentTrafficSystem/Blueprints/Pedestrian_BPs/BP_Pedestrian.BP_Pedestrian_C|GetActive%20Path (Variables|Default|GetAs%20BP%20Pedestrian))) 5e+01 "World"))
      (AI|BehaviorTree|FinishExecute true)
      (else
        (AI|BehaviorTree|SetBlackboardValueasVector (Variables|Default|GetTarget%20location) (Spline|GetLocationatDistanceAlongSpline (Variables|/Game/IntelligentTrafficSystem/Blueprints/Pedestrian_BPs/BP_PedestrianPath.BP_PedestrianPath_C|GetSpline (Variables|/Game/IntelligentTrafficSystem/Blueprints/Pedestrian_BPs/BP_Pedestrian.BP_Pedestrian_C|GetActive%20Path (Variables|Default|GetAs%20BP%20Pedestrian))) (- (Spline|GetSplineLength (Variables|/Game/IntelligentTrafficSystem/Blueprints/Pedestrian_BPs/BP_PedestrianPath.BP_PedestrianPath_C|GetSpline (Variables|/Game/IntelligentTrafficSystem/Blueprints/Pedestrian_BPs/BP_Pedestrian.BP_Pedestrian_C|GetActive%20Path (Variables|Default|GetAs%20BP%20Pedestrian)))) 5e+01) "World"))
        (AI|BehaviorTree|FinishExecute true)))
    (elif (Variables|/Game/IntelligentTrafficSystem/Blueprints/Pedestrian_BPs/BP_Pedestrian.BP_Pedestrian_C|GetForward? (Variables|Default|GetAs%20BP%20Pedestrian))
      (for (_array_element _array_index) (Variables|/Game/IntelligentTrafficSystem/Blueprints/Pedestrian_BPs/BP_Pedestrian.BP_Pedestrian_C|GetNext%20Path (Variables|Default|GetAs%20BP%20Pedestrian))
        (if (< (Math|Vector|Distance(Vector) (Spline|GetLocationatDistanceAlongSpline (Variables|/Game/IntelligentTrafficSystem/Blueprints/Pedestrian_BPs/BP_PedestrianPath.BP_PedestrianPath_C|GetSpline _array_element) 0.0 "World") (Transformation|GetActorLocation (Variables|Default|GetAs%20BP%20Pedestrian))) 2e+03)
          (Utilities|Array|Insert _paths_to_switch_2 _array_element _array_index)
          (else
            (Utilities|Array|RemoveItem _paths_to_switch_2 _array_element)))
        (AI|BehaviorTree|FinishExecute true))
      (bind _output_get_2 (Variables|/Game/IntelligentTrafficSystem/Blueprints/Pedestrian_BPs/BP_Pedestrian.BP_Pedestrian_C|SetActive%20Path (Variables|Default|GetAs%20BP%20Pedestrian) (.OutItem (Utilities|Array|Random (Variables|Default|GetPaths%20to%20switch)))))
      (AI|AIMoveTo (Variables|Default|GetAs%20BP%20Pedestrian) (Spline|GetLocationatDistanceAlongSpline (Variables|/Game/IntelligentTrafficSystem/Blueprints/Pedestrian_BPs/BP_PedestrianPath.BP_PedestrianPath_C|GetSpline _output_get_2) 0.0 "World") 0 5.0 false
        (:OnSuccess
          (AI|BehaviorTree|FinishExecute true)))
      (else
        (for (_array_element_2 _array_index_2) (Variables|/Game/IntelligentTrafficSystem/Blueprints/Pedestrian_BPs/BP_Pedestrian.BP_Pedestrian_C|GetNext%20Path (Variables|Default|GetAs%20BP%20Pedestrian))
          (if (< (Math|Vector|Distance(Vector) (Spline|GetLocationatDistanceAlongSpline (Variables|/Game/IntelligentTrafficSystem/Blueprints/Pedestrian_BPs/BP_PedestrianPath.BP_PedestrianPath_C|GetSpline _array_element_2) (Spline|GetSplineLength (Variables|/Game/IntelligentTrafficSystem/Blueprints/Pedestrian_BPs/BP_PedestrianPath.BP_PedestrianPath_C|GetSpline _array_element_2)) "World") (Transformation|GetActorLocation (Variables|Default|GetAs%20BP%20Pedestrian))) 2e+03)
            (Utilities|Array|Insert _paths_to_switch _array_element_2 _array_index_2)
            (else
              (Utilities|Array|RemoveItem _paths_to_switch _array_element_2)))
          (AI|BehaviorTree|FinishExecute true))
        (Variables|/Game/IntelligentTrafficSystem/Blueprints/Pedestrian_BPs/BP_Pedestrian.BP_Pedestrian_C|SetActive%20Path (Variables|Default|GetAs%20BP%20Pedestrian) (.OutItem (Utilities|Array|Random (Variables|Default|GetPaths%20to%20switch))))
        (Default|MoveAlongPath (Variables|Default|GetAs%20BP%20Pedestrian))
        (AI|BehaviorTree|FinishExecute true)))))