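; Behavior tree task that sends a traffic-system pedestrian toward its road-crossing target.
; It copies the pedestrian controller's Stop flag and the pawn's CrossingTargetLocation actor into the Stop and Target blackboard keys.
; It then issues AIMoveTo to that actor's location and finishes successfully on the immediate exec output, without waiting for arrival.
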(event EventReceiveExecuteAI
  (params (OwnerController :type AI%20Controller%20Object%20Reference) (ControlledPawn :type Pawn%20Object%20Reference))
  (bind _asbp_pedestrian (Utilities|Casting|CastToBP_Pedestrian ControlledPawn))
  (bind _asaic_pedestrian_controller (Utilities|Casting|CastToAIC_PedestrianController OwnerController))
  (Class|BTFunctionLibrary|SetBlackboardValueasBool (Variables|Default|GetStop) (Variables|/Game/IntelligentTrafficSystem/Blueprints/Pedestrian_BPs/AIC_PedestrianController.AIC_PedestrianController_C|GetStop _asaic_pedestrian_controller))
  (Class|BTFunctionLibrary|SetBlackboardValueasObject (Variables|Default|GetTarget) (Variables|/Game/IntelligentTrafficSystem/Blueprints/Pedestrian_BPs/BP_Pedestrian.BP_Pedestrian_C|GetCrossing%20Target%20location _asbp_pedestrian))
  (AI|AIMoveTo _asbp_pedestrian (Transformation|GetActorLocation (Variables|/Game/IntelligentTrafficSystem/Blueprints/Pedestrian_BPs/BP_Pedestrian.BP_Pedestrian_C|GetCrossing%20Target%20location _asbp_pedestrian)) 0 5.0 false
    (:then
      (AI|BehaviorTree|FinishExecute true))))