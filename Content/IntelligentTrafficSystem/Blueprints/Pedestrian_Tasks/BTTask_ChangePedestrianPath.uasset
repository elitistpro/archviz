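; Behavior tree task that moves a BP_Pedestrian onto a connected path when it reaches the end of its spline.
; Looped paths just clear ReachedSplineEnd; otherwise it picks a random NextPath whose direction-matching end is nearer and within range, then walks there with AIMoveTo.
; With no candidate it flips the pedestrian's Forward flag and finishes.
; A nearest-path fallback event exists, but its calls are disconnected.
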(event Custom|Change%20Path%20when%20deafult%20option%20fails
  (params (Forward :type Boolean) (Backward :type Boolean))
  (bind _as_bp_pedestrian (Variables|Default|GetAs%20BP%20Pedestrian))
  (bind _as_bp_pedestrian_2 (Variables|Default|GetAs%20BP%20Pedestrian))
  (bind _as_bp_pedestrian_3 (Variables|Default|GetAs%20BP%20Pedestrian))
  (bind _returnvalue (Transformation|GetActorLocation _as_bp_pedestrian_2))
  (if (and Forward Backward)
    (if (< (Math|Vector|Distance(Vector) (Spline|GetLocationatSplinePoint (Variables|/Game/IntelligentTrafficSystem/Blueprints/Pedestrian_BPs/BP_PedestrianPath.BP_PedestrianPath_C|GetSpline (.AsBP%20Pedestrian%20Path (Utilities|Casting|CastToBP_PedestrianPath (.ReturnValue (Actor|FindNearestActor (Transformation|GetActorLocation _as_bp_pedestrian) (Variables|/Game/IntelligentTrafficSystem/Blueprints/Pedestrian_BPs/BP_PedestrianPath.BP_PedestrianPath_C|GetNext%20Path (Variables|/Game/IntelligentTrafficSystem/Blueprints/Pedestrian_BPs/BP_Pedestrian.BP_Pedestrian_C|GetActive%20Path _as_bp_pedestrian))))))) 0 "World") _returnvalue) (Math|Vector|Distance(Vector) (Spline|GetLocationatSplinePoint (Variables|/Game/IntelligentTrafficSystem/Blueprints/Pedestrian_BPs/BP_PedestrianPath.BP_PedestrianPath_C|GetSpline (.AsBP%20Pedestrian%20Path (Utilities|Casting|CastToBP_PedestrianPath (.ReturnValue (Actor|FindNearestActor (Transformation|GetActorLocation _as_bp_pedestrian) (Variables|/Game/IntelligentTrafficSystem/Blueprints/Pedestrian_BPs/BP_PedestrianPath.BP_PedestrianPath_C|GetNext%20Path (Variables|/Game/IntelligentTrafficSystem/Blueprints/Pedestrian_BPs/BP_Pedestrian.BP_Pedestrian_C|GetActive%20Path _as_bp_pedestrian))))))) (- (Spline|GetNumberOfSplinePoints (Variables|/Game/IntelligentTrafficSystem/Blueprints/Pedestrian_BPs/BP_PedestrianPath.BP_PedestrianPath_C|GetSpline (.AsBP%20Pedestrian%20Path (Utilities|Casting|CastToBP_PedestrianPath (.ReturnValue (Actor|FindNearestActor (Transformation|GetActorLocation _as_bp_pedestrian) (Variables|/Game/IntelligentTrafficSystem/Blueprints/Pedestrian_BPs/BP_PedestrianPath.BP_PedestrianPath_C|GetNext%20Path (Variables|/Game/IntelligentTrafficSystem/Blueprints/Pedestrian_BPs/BP_Pedestrian.BP_Pedestrian_C|GetActive%20Path _as_bp_pedestrian)))))))) 1) "World") _returnvalue))
      (Variables|/Game/IntelligentTrafficSystem/Blueprints/Pedestrian_BPs/BP_Pedestrian.BP_Pedestrian_C|SetForward? _as_bp_pedestrian_3 true)
      (else
        (Variables|/Game/IntelligentTrafficSystem/Blueprints/Pedestrian_BPs/BP_Pedestrian.BP_Pedestrian_C|SetForward? _as_bp_pedestrian_3 false)))
    (Variables|/Game/IntelligentTrafficSystem/Blueprints/Pedestrian_BPs/BP_Pedestrian.BP_Pedestrian_C|SetActive%20Path (Variables|Default|GetAs%20BP%20Pedestrian) (.AsBP%20Pedestrian%20Path (Utilities|Casting|CastToBP_PedestrianPath (.ReturnValue (Actor|FindNearestActor (Transformation|GetActorLocation _as_bp_pedestrian) (Variables|/Game/IntelligentTrafficSystem/Blueprints/Pedestrian_BPs/BP_PedestrianPath.BP_PedestrianPath_C|GetNext%20Path (Variables|/Game/IntelligentTrafficSystem/Blueprints/Pedestrian_BPs/BP_Pedestrian.BP_Pedestrian_C|GetActive%20Path _as_bp_pedestrian)))))))
    (Class|BTFunctionLibrary|SetBlackboardValueasBool (Variables|Default|GetReached%20Spline%20End) false)))

(event EventReceiveExecuteAI
  (params (OwnerController :type AI%20Controller%20Object%20Reference) (ControlledPawn :type Pawn%20Object%20Reference))
  (bind _available_paths (Variables|Default|GetAvailable%20paths))
  (bind _available_paths_2 (Variables|Default|GetAvailable%20paths))
  (bind _outitem (Utilities|Array|Random _available_paths))
  (bind _outitem_2 (Utilities|Array|Random _available_paths_2))
  (bind _asbp_pedestrian (Utilities|Casting|CastToBP_Pedestrian ControlledPawn))
  (bind _output_get (Variables|Default|SetAs%20BP%20Pedestrian _asbp_pedestrian))
  (Variables|/Game/IntelligentTrafficSystem/Blueprints/Pedestrian_BPs/BP_Pedestrian.BP_Pedestrian_C|SetChanging%20Paths _asbp_pedestrian true)
  (if (Variables|/Game/IntelligentTrafficSystem/Blueprints/Pedestrian_BPs/BP_PedestrianPath.BP_PedestrianPath_C|GetLoop? (Variables|/Game/IntelligentTrafficSystem/Blueprints/Pedestrian_BPs/BP_Pedestrian.BP_Pedestrian_C|GetActive%20Path _output_get))
    (Class|BTFunctionLibrary|SetBlackboardValueasBool (Variables|Default|GetReached%20Spline%20End) false)
    (AI|BehaviorTree|FinishExecute true)
    (elif (Variables|/Game/IntelligentTrafficSystem/Blueprints/Pedestrian_BPs/BP_Pedestrian.BP_Pedestrian_C|GetForward? (Variables|Default|GetAs%20BP%20Pedestrian))
      (for _array_element (Variables|/Game/IntelligentTrafficSystem/Blueprints/Pedestrian_BPs/BP_PedestrianPath.BP_PedestrianPath_C|GetNext%20Path (Variables|/Game/IntelligentTrafficSystem/Blueprints/Pedestrian_BPs/BP_Pedestrian.BP_Pedestrian_C|GetActive%20Path (Variables|Default|GetAs%20BP%20Pedestrian)))
        (if (< (Math|Vector|Distance(Vector) (Transformation|GetActorLocation (Variables|Default|GetAs%20BP%20Pedestrian)) (Spline|GetLocationatDistanceAlongSpline (Variables|/Game/IntelligentTrafficSystem/Blueprints/Pedestrian_BPs/BP_PedestrianPath.BP_PedestrianPath_C|GetSpline _array_element) 0.0 "World")) (Math|Vector|Distance(Vector) (Transformation|GetActorLocation (Variables|Default|GetAs%20BP%20Pedestrian)) (Spline|GetLocationatDistanceAlongSpline (Variables|/Game/IntelligentTrafficSystem/Blueprints/Pedestrian_BPs/BP_PedestrianPath.BP_PedestrianPath_C|GetSpline _array_element) (Spline|GetSplineLength (Variables|/Game/IntelligentTrafficSystem/Blueprints/Pedestrian_BPs/BP_PedestrianPath.BP_PedestrianPath_C|GetSpline _array_element)) "World")))
          (if (< (Math|Vector|Distance(Vector) (Transformation|GetActorLocation (Variables|Default|GetAs%20BP%20Pedestrian)) (Spline|GetLocationatDistanceAlongSpline (Variables|/Game/IntelligentTrafficSystem/Blueprints/Pedestrian_BPs/BP_PedestrianPath.BP_PedestrianPath_C|GetSpline _array_element) 0.0 "World")) 1e+03)
            (Utilities|Array|Add (Variables|Default|GetAvailable%20paths) _array_element))))
      (Utilities|IsValid _outitem_2
        (:Is%20Valid
          (bind _output_get_2 (Variables|Default|SetChosen%20path _outitem_2))
          (bind _output_get_3 (Variables|/Game/IntelligentTrafficSystem/Blueprints/Pedestrian_BPs/BP_Pedestrian.BP_Pedestrian_C|SetActive%20Path (Variables|Default|GetAs%20BP%20Pedestrian) _output_get_2))
          (Variables|Default|SetForwad%20Fail false)
          (AI|AIMoveTo (Variables|Default|GetAs%20BP%20Pedestrian) (Spline|GetLocationatDistanceAlongSpline (Variables|/Game/IntelligentTrafficSystem/Blueprints/Pedestrian_BPs/BP_PedestrianPath.BP_PedestrianPath_C|GetSpline _output_get_3) 0.0 "World") 0 1e+02 false
            (:OnSuccess
              (Class|BTFunctionLibrary|SetBlackboardValueasBool (Variables|Default|GetReached%20Spline%20End) false)
              (Utilities|Array|Clear (Variables|Default|GetAvailable%20paths))
              (AI|BehaviorTree|FinishExecute true))))
        (:Is%20Not%20Valid
          (Utilities|Array|Clear (Variables|Default|GetAvailable%20paths))
          (Variables|/Game/IntelligentTrafficSystem/Blueprints/Pedestrian_BPs/BP_Pedestrian.BP_Pedestrian_C|SetForward? (Variables|Default|GetAs%20BP%20Pedestrian) false)
          (bind _output_get_4 (Variables|Default|SetForwad%20Fail true))
          (AI|BehaviorTree|FinishExecute true)))
      (else
        (for _array_element_2 (Variables|/Game/IntelligentTrafficSystem/Blueprints/Pedestrian_BPs/BP_PedestrianPath.BP_PedestrianPath_C|GetNext%20Path (Variables|/Game/IntelligentTrafficSystem/Blueprints/Pedestrian_BPs/BP_Pedestrian.BP_Pedestrian_C|GetActive%20Path (Variables|Default|GetAs%20BP%20Pedestrian)))
          (if (not (< (Math|Vector|Distance(Vector) (Transformation|GetActorLocation (Variables|Default|GetAs%20BP%20Pedestrian)) (Spline|GetLocationatDistanceAlongSpline (Variables|/Game/IntelligentTrafficSystem/Blueprints/Pedestrian_BPs/BP_PedestrianPath.BP_PedestrianPath_C|GetSpline _array_element_2) 0.0 "World")) (Math|Vector|Distance(Vector) (Transformation|GetActorLocation (Variables|Default|GetAs%20BP%20Pedestrian)) (Spline|GetLocationatDistanceAlongSpline (Variables|/Game/IntelligentTrafficSystem/Blueprints/Pedestrian_BPs/BP_PedestrianPath.BP_PedestrianPath_C|GetSpline _array_element_2) (Spline|GetSplineLength (Variables|/Game/IntelligentTrafficSystem/Blueprints/Pedestrian_BPs/BP_PedestrianPath.BP_PedestrianPath_C|GetSpline _array_element_2)) "World"))))
            (if (< (Math|Vector|Distance(Vector) (Transformation|GetActorLocation (Variables|Default|GetAs%20BP%20Pedestrian)) (Spline|GetLocationatDistanceAlongSpline (Variables|/Game/IntelligentTrafficSystem/Blueprints/Pedestrian_BPs/BP_PedestrianPath.BP_PedestrianPath_C|GetSpline _array_element_2) (Spline|GetSplineLength (Variables|/Game/IntelligentTrafficSystem/Blueprints/Pedestrian_BPs/BP_PedestrianPath.BP_PedestrianPath_C|GetSpline _array_element_2)) "World")) 1e+03)
              (Utilities|Array|Add (Variables|Default|GetAvailable%20paths) _array_element_2))))
        (Utilities|IsValid _outitem
          (:Is%20Valid
            (bind _output_get_5 (Variables|Default|SetChosen%20path _outitem))
            (bind _output_get_6 (Variables|/Game/IntelligentTrafficSystem/Blueprints/Pedestrian_BPs/BP_Pedestrian.BP_Pedestrian_C|SetActive%20Path (Variables|Default|GetAs%20BP%20Pedestrian) _output_get_5))
            (Variables|Default|SetBackward%20Fail false)
            (AI|AIMoveTo (Variables|Default|GetAs%20BP%20Pedestrian) (Spline|GetLocationatDistanceAlongSpline (Variables|/Game/IntelligentTrafficSystem/Blueprints/Pedestrian_BPs/BP_PedestrianPath.BP_PedestrianPath_C|GetSpline _output_get_6) (Spline|GetSplineLength (Variables|/Game/IntelligentTrafficSystem/Blueprints/Pedestrian_BPs/BP_PedestrianPath.BP_PedestrianPath_C|GetSpline _output_get_6)) "World") 0 1e+02 false
              (:OnSuccess
                (Class|BTFunctionLibrary|SetBlackboardValueasBool (Variables|Default|GetReached%20Spline%20End) false)
                (Utilities|Array|Clear (Variables|Default|GetAvailable%20paths))
                (AI|BehaviorTree|FinishExecute true))))
          (:Is%20Not%20Valid
            (Utilities|Array|Clear (Variables|Default|GetAvailable%20paths))
            (Variables|/Game/IntelligentTrafficSystem/Blueprints/Pedestrian_BPs/BP_Pedestrian.BP_Pedestrian_C|SetForward? (Variables|Default|GetAs%20BP%20Pedestrian) true)
            (bind _output_get_7 (Variables|Default|SetBackward%20Fail true))
            (AI|BehaviorTree|FinishExecute true)))))))