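; Behavior tree task that walks a BP_Pedestrian along its active path spline in its Forward or reverse direction.
; It clears ChangingPaths, then flags ReachedSplineEnd on the blackboard if the pawn is near that direction's end.
; Otherwise it sets walk speed and calls AIMoveTo toward a tangent look-ahead point snapped back onto the spline.
; The task finishes as soon as the move is issued, without waiting for arrival.
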(event EventReceiveExecuteAI
  (params (OwnerController :type AI%20Controller%20Object%20Reference) (ControlledPawn :type Pawn%20Object%20Reference))
  (bind _asbp_pedestrian (Utilities|Casting|CastToBP_Pedestrian ControlledPawn))
  (bind _output_get (Variables|Default|SetAs%20BP%20Pedestrian _asbp_pedestrian))
  (Variables|/Game/IntelligentTrafficSystem/Blueprints/Pedestrian_BPs/BP_Pedestrian.BP_Pedestrian_C|SetChanging%20Paths _asbp_pedestrian false)
  (if (Variables|/Game/IntelligentTrafficSystem/Blueprints/Pedestrian_BPs/BP_Pedestrian.BP_Pedestrian_C|GetForward? _output_get)
    (if (< (Math|Vector|Distance(Vector) (Spline|GetLocationatDistanceAlongSpline (Variables|/Game/IntelligentTrafficSystem/Blueprints/Pedestrian_BPs/BP_PedestrianPath.BP_PedestrianPath_C|GetSpline (Variables|/Game/IntelligentTrafficSystem/Blueprints/Pedestrian_BPs/BP_Pedestrian.BP_Pedestrian_C|GetActive%20Path (Variables|Default|GetAs%20BP%20Pedestrian))) (Spline|GetSplineLength (Variables|/Game/IntelligentTrafficSystem/Blueprints/Pedestrian_BPs/BP_PedestrianPath.BP_PedestrianPath_C|GetSpline (Variables|/Game/IntelligentTrafficSystem/Blueprints/Pedestrian_BPs/BP_Pedestrian.BP_Pedestrian_C|GetActive%20Path (Variables|Default|GetAs%20BP%20Pedestrian)))) "World") (Transformation|GetActorLocation (Variables|Default|GetAs%20BP%20Pedestrian))) 1e+02)
      (Class|BTFunctionLibrary|SetBlackboardValueasBool (Variables|Default|GetReached%20Spline%20End) true)
      (AI|BehaviorTree|FinishExecute true)
      (else
        (Variables|/Script/Engine.CharacterMovementComponent|SetMaxWalkSpeed (Variables|/Script/Engine.Character|GetCharacterMovement (Variables|Default|GetAs%20BP%20Pedestrian)) (Variables|Default|GetMax%20Walk%20Speed))
        (AI|AIMoveTo (Variables|Default|GetAs%20BP%20Pedestrian) (Spline|FindLocationClosesttoWorldLocation (Variables|/Game/IntelligentTrafficSystem/Blueprints/Pedestrian_BPs/BP_PedestrianPath.BP_PedestrianPath_C|GetSpline (Variables|/Game/IntelligentTrafficSystem/Blueprints/Pedestrian_BPs/BP_Pedestrian.BP_Pedestrian_C|GetActive%20Path (Variables|Default|GetAs%20BP%20Pedestrian))) (+ (* (Math|Vector|Normalize (Class|SplineComponent|FindTangentClosesttoWorldLocation (Variables|/Game/IntelligentTrafficSystem/Blueprints/Pedestrian_BPs/BP_PedestrianPath.BP_PedestrianPath_C|GetSpline (Variables|/Game/IntelligentTrafficSystem/Blueprints/Pedestrian_BPs/BP_Pedestrian.BP_Pedestrian_C|GetActive%20Path (Variables|Default|GetAs%20BP%20Pedestrian))) (Transformation|GetActorLocation (Variables|Default|GetAs%20BP%20Pedestrian)) "World")) 6e+02) (Transformation|GetActorLocation (Variables|Default|GetAs%20BP%20Pedestrian))) "World") 0 5e+01 false
          (:then
            (AI|BehaviorTree|FinishExecute true :!label _label))
          (:OnSuccess
            (goto _label))
          (:OnFail
            (Class|BTTaskBlueprintBase|FinishAbort)))))
    (elif (< (Math|Vector|Distance(Vector) (Spline|GetLocationatDistanceAlongSpline (Variables|/Game/IntelligentTrafficSystem/Blueprints/Pedestrian_BPs/BP_PedestrianPath.BP_PedestrianPath_C|GetSpline (Variables|/Game/IntelligentTrafficSystem/Blueprints/Pedestrian_BPs/BP_Pedestrian.BP_Pedestrian_C|GetActive%20Path (Variables|Default|GetAs%20BP%20Pedestrian))) 0.0 "World") (Transformation|GetActorLocation (Variables|Default|GetAs%20BP%20Pedestrian))) 1e+02)
      (Class|BTFunctionLibrary|SetBlackboardValueasBool (Variables|Default|GetReached%20Spline%20End) true)
      (AI|BehaviorTree|FinishExecute true)
      (else
        (Variables|/Script/Engine.CharacterMovementComponent|SetMaxWalkSpeed (Variables|/Script/Engine.Character|GetCharacterMovement (Variables|Default|GetAs%20BP%20Pedestrian)) (Variables|Default|GetMax%20Walk%20Speed))
        (AI|AIMoveTo (Variables|Default|GetAs%20BP%20Pedestrian) (Spline|FindLocationClosesttoWorldLocation (Variables|/Game/IntelligentTrafficSystem/Blueprints/Pedestrian_BPs/BP_PedestrianPath.BP_PedestrianPath_C|GetSpline (Variables|/Game/IntelligentTrafficSystem/Blueprints/Pedestrian_BPs/BP_Pedestrian.BP_Pedestrian_C|GetActive%20Path (Variables|Default|GetAs%20BP%20Pedestrian))) (- (Transformation|GetActorLocation (Variables|Default|GetAs%20BP%20Pedestrian)) (* (Math|Vector|Normalize (Class|SplineComponent|FindTangentClosesttoWorldLocation (Variables|/Game/IntelligentTrafficSystem/Blueprints/Pedestrian_BPs/BP_PedestrianPath.BP_PedestrianPath_C|GetSpline (Variables|/Game/IntelligentTrafficSystem/Blueprints/Pedestrian_BPs/BP_Pedestrian.BP_Pedestrian_C|GetActive%20Path (Variables|Default|GetAs%20BP%20Pedestrian))) (Transformation|GetActorLocation (Variables|Default|GetAs%20BP%20Pedestrian)) "World")) 6e+02)) "World") 0 5e+01 false
          (:then
            (AI|BehaviorTree|FinishExecute true :!label _label_2))
          (:OnSuccess
            (goto _label_2))
          (:OnFail
            (Class|BTTaskBlueprintBase|FinishAbort)))))))