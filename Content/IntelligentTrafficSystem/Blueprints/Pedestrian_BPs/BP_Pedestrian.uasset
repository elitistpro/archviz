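; BP_Pedestrian is an AI pedestrian that walks along a path spline in a random starting direction, with randomized cap, shirt and jeans materials.
; It feeds spline look-ahead targets to its controller's blackboard and reverses after a countdown at the spline end.
; It walks when the nearest traffic light's Stop flag is set, otherwise halts.
; When ragdolled by a car, it requests a replacement spawn from pedestrian paths and destroys itself.
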(event Custom|Move%20along%20path
  (bind _returnvalue (Transformation|GetActorLocation))
  (bind _active_path (Variables|Default|GetActive%20Path))
  (bind _spline (Variables|/Game/IntelligentTrafficSystem/Blueprints/Pedestrian_BPs/BP_PedestrianPath.BP_PedestrianPath_C|GetSpline _active_path))
  (bind _returnvalue_2 (Class|SplineComponent|FindTangentClosesttoWorldLocation _spline _returnvalue "World"))
  (bind _returnvalue_3 (Math|Vector|Normalize _returnvalue_2))
  (bind _returnvalue_4 (* _returnvalue_3 1e+02))
  ;[1 1 1] Move Along Spline
  (bind _asaic_pedestrian_controller (Utilities|Casting|CastToAIC_PedestrianController (Pawn|GetController)))
  (if (Variables|Default|GetForward?)
    (bind _output_get (Variables|Default|SetTarget%20Location (Spline|FindLocationClosesttoWorldLocation _spline (+ _returnvalue_4 _returnvalue) "World")))
    (AI|Components|Blackboard|SetValueasVector (AI|GetBlackboard _asaic_pedestrian_controller) (Utilities|Name|MakeLiteralName "Target Location") _output_get)
    (else
      (bind _output_get_2 (Variables|Default|SetTarget%20Location (Spline|FindLocationClosesttoWorldLocation _spline (- _returnvalue _returnvalue_4) "World")))
      (AI|Components|Blackboard|SetValueasVector (AI|GetBlackboard _asaic_pedestrian_controller) (Utilities|Name|MakeLiteralName "Target Location") _output_get_2))))

(event Custom|Traffic%20light%20response
  (bind _charactermovement (Variables|Character|GetCharacterMovement))
  ;[1 1 1] Traffic Light REsponse
  (bind _outactors (Actor|GetAllActorsOfClass "/Game/IntelligentTrafficSystem/Blueprints/Vehicle_BPs/BP_TrafficLight.BP_TrafficLight_C"))
  (bind _asbp_traffic_light (Utilities|Casting|CastToBP_TrafficLight (.ReturnValue (Actor|FindNearestActor (Transformation|GetActorLocation) _outactors))))
  (if (Variables|/Game/IntelligentTrafficSystem/Blueprints/Vehicle_BPs/BP_TrafficLight.BP_TrafficLight_C|GetStop _asbp_traffic_light)
    (Variables|/Script/Engine.CharacterMovementComponent|SetMaxWalkSpeed _charactermovement 2.5e+02)
    (else
      (Variables|/Script/Engine.CharacterMovementComponent|SetMaxWalkSpeed _charactermovement 0.0))))

(event Custom|Ragdoll
  (params (Car :type BP%20Ai%20Car%20Object%20Reference))
  ;[1 1 1] Ragdoll
  (bind _output_get (Variables|Default|SetCar Car))
  (AI|Navigation|StopMovement (Pawn|GetController))
  (Physics|SetSimulatePhysics (Variables|Character|GetMesh) true)
  (Utilities|FlowControl|Delay 1.5)
  (bind _outactors (Actor|GetAllActorsOfClass "/Game/IntelligentTrafficSystem/Blueprints/Pedestrian_BPs/BP_PedestrianPath.BP_PedestrianPath_C"))
  (for _array_element _outactors
    (if (Variables|/Game/IntelligentTrafficSystem/Blueprints/Pedestrian_BPs/BP_PedestrianPath.BP_PedestrianPath_C|GetSpawn%20Pedestrians? _array_element)
      (Utilities|FlowControl|DoOnce false
        (:Completed
          (Variables|/Game/IntelligentTrafficSystem/Blueprints/Pedestrian_BPs/BP_PedestrianPath.BP_PedestrianPath_C|SetNumber%20of%20pedestrians%20to%20spawn (.OutItem (Utilities|Array|Random _outactors)) (+ (Variables|/Game/IntelligentTrafficSystem/Blueprints/Pedestrian_BPs/BP_PedestrianPath.BP_PedestrianPath_C|GetNumber%20of%20pedestrians%20to%20spawn (.OutItem (Utilities|Array|Random _outactors))) 1))
          (Actor|DestroyActor))))))

(event Custom|Changing%20Path%20Timer
  (if (< (Variables|Default|Getchanging%20Path%20Time) 0)
    (if (Variables|Default|GetForward?)
      (Variables|Default|SetForward? false)
      (else
        (Variables|Default|SetForward? true)))
    (AI|Components|Blackboard|SetValueasBool (AI|GetBlackboard 0) (Utilities|Name|MakeLiteralName "Reached Spline End") false)
    (Variables|Default|Setchanging%20Path%20Time 5)
    (elif (ScalableFloat|GetValueasBool (AI|GetBlackboard 0) (Utilities|Name|MakeLiteralName "Reached Spline End"))
      (Utilities|FlowControl|Delay 1.0)
      (bind _output_get (Variables|Default|Setchanging%20Path%20Time (- (Variables|Default|Getchanging%20Path%20Time) 1)))
      (Development|PrintString (Utilities|String|ToString(Integer) _output_get))
      (CallFunction|ChangingPathTimer)
      (else
        (Variables|Default|Setchanging%20Path%20Time 5)))))

(event EventBeginPlay
  ;[1 1 1] Beginplay
  (Utilities|FlowControl|Sequence
    (:then_0
      (Variables|/Script/Engine.SkinnedMeshComponent|SetVisibilityBasedAnimTickOption (Variables|Character|GetMesh) "AlwaysTickPoseAndRefreshBones"))
    (:then_1
      (switch int (Math|Random|RandomIntegerinRange 0 1)
        (:0
          (Variables|Default|SetForward? true))
        (:1
          (Variables|Default|SetForward? false))))
    (:then_2
      (Rendering|Material|SetMaterial (Variables|Default|GetCharacterMesh2) 1 (.OutItem (Utilities|Array|Random (Variables|Default|GetCapMaterial))))
      (Rendering|Material|SetMaterial (Variables|Default|GetCharacterMesh2) 5 (.OutItem (Utilities|Array|Random (Variables|Default|GetShirtMaterial))))
      (Rendering|Material|SetMaterial (Variables|Default|GetCharacterMesh2) 7 (.OutItem (Utilities|Array|Random (Variables|Default|GetJeansMaterial)))))))

(fn ConstructionScript)

(fn FindImpulsDirection)

(fn SwitchPaths
  (if (Variables|Default|GetReached%20Spline%20End)
    _))