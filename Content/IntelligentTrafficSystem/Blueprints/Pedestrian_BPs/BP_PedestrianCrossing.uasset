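; Pedestrian crossing trigger for the traffic system that tells AI pedestrians when to wait and where to cross.
; Tick, throttled by a Delay, checks overlapping traffic lights and clears overlapping pedestrians' "Stop at Traffic light" blackboard flag when Stop is true, otherwise sets it.
; Box overlap either sets a random crossing target and "Cross the Road" (the random branch always picks crossing), or, if already crossing, assigns a random CrossingPath and clears it.
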(event OnComponentBeginOverlap(Box)
  (params (OverlappedComponent :type Primitive%20Component%20Object%20Reference) (OtherActor :type Actor%20Object%20Reference) (OtherComp :type Primitive%20Component%20Object%20Reference) (OtherBodyIndex :type Integer) (bFromSweep :type Boolean) (SweepResult :type Hit%20Result%20Structure%20%28by%20ref%29))
  (bind _asbp_pedestrian (Utilities|Casting|CastToBP_Pedestrian OtherActor))
  (if (ScalableFloat|GetValueasBool (AI|GetBlackboard (.AsAIC%20Pedestrian%20Controller (Utilities|Casting|CastToAIC_PedestrianController (Pawn|GetController _asbp_pedestrian)))) (Utilities|Name|MakeLiteralName "Cross the Road"))
    (Variables|/Game/IntelligentTrafficSystem/Blueprints/Pedestrian_BPs/BP_Pedestrian.BP_Pedestrian_C|SetActive%20Path _asbp_pedestrian (.OutItem (Utilities|Array|Random (Variables|Default|GetCrossing%20Path))))
    (bind _asaic_pedestrian_controller (Utilities|Casting|CastToAIC_PedestrianController (Pawn|GetController _asbp_pedestrian)))
    (AI|Components|Blackboard|SetValueasBool (AI|GetBlackboard _asaic_pedestrian_controller) (Utilities|Name|MakeLiteralName "Cross the Road") false)
    (else
      (Variables|/Game/IntelligentTrafficSystem/Blueprints/Pedestrian_BPs/BP_Pedestrian.BP_Pedestrian_C|SetCrossing%20Target%20location _asbp_pedestrian (.OutItem (Utilities|Array|Random (Variables|Default|GetCrossing%20Target%20location))))
      (switch int (Math|Random|RandomIntegerinRange 0 0)
        (:0
          (bind _asaic_pedestrian_controller_2 (Utilities|Casting|CastToAIC_PedestrianController (Pawn|GetController _asbp_pedestrian)))
          (AI|Components|Blackboard|SetValueasBool (AI|GetBlackboard _asaic_pedestrian_controller_2) (Utilities|Name|MakeLiteralName "Cross the Road") true))
        (:1
          (bind _asaic_pedestrian_controller_3 (Utilities|Casting|CastToAIC_PedestrianController (Pawn|GetController _asbp_pedestrian) :!label _label))
          (AI|Components|Blackboard|SetValueasBool (AI|GetBlackboard _asaic_pedestrian_controller_3) (Utilities|Name|MakeLiteralName "Cross the Road") false))
        (:2
          (goto _label))))))

(event EventBeginPlay)

(event EventTick
  (params (DeltaSeconds :type Float%20%28single-precision%29))
  (bind _overlappingactors (Collision|GetOverlappingActors "/Game/IntelligentTrafficSystem/Blueprints/Pedestrian_BPs/BP_Pedestrian.BP_Pedestrian_C" :!class /Script/Engine.Actor))
  (Utilities|FlowControl|Delay 0.5)
  (for _array_element (Collision|GetOverlappingActors "/Game/IntelligentTrafficSystem/Blueprints/Vehicle_BPs/BP_TrafficLight.BP_TrafficLight_C" :!class /Script/Engine.Actor)
    (bind _asbp_traffic_light (Utilities|Casting|CastToBP_TrafficLight _array_element))
    (if (Variables|/Game/IntelligentTrafficSystem/Blueprints/Vehicle_BPs/BP_TrafficLight.BP_TrafficLight_C|GetStop _asbp_traffic_light)
      (for _array_element_2 _overlappingactors
        (Utilities|IsValid _array_element_2
          (:Is%20Valid
            (bind _asbp_pedestrian (Utilities|Casting|CastToBP_Pedestrian _array_element_2))
            (bind _asaic_pedestrian_controller (Utilities|Casting|CastToAIC_PedestrianController (Pawn|GetController _asbp_pedestrian)))
            (AI|Components|Blackboard|SetValueasBool (AI|GetBlackboard _asaic_pedestrian_controller) (Utilities|Name|MakeLiteralName "Stop at Traffic light") false))))
      (else
        (for _array_element_3 _overlappingactors
          (Utilities|IsValid _array_element_3
            (:Is%20Valid
              (bind _asbp_pedestrian_2 (Utilities|Casting|CastToBP_Pedestrian _array_element_3))
              (bind _asaic_pedestrian_controller_2 (Utilities|Casting|CastToAIC_PedestrianController (Pawn|GetController _asbp_pedestrian_2)))
              (AI|Components|Blackboard|SetValueasBool (AI|GetBlackboard _asaic_pedestrian_controller_2) (Utilities|Name|MakeLiteralName "Stop at Traffic light") true))))))))

(fn ConstructionScript)