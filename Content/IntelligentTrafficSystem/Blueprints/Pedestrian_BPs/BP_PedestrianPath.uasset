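; Spline path actor for pedestrians in the traffic system that can populate itself with walking AI.
; On BeginPlay, if enabled, it spawns BP_Pedestrian pawns running BT_Pedestrian one per second until the count runs out, using a self-calling delayed event.
; Each spawns at a random distance along the spline and takes this actor as its active path.
; A SnaptoGround event line-traces each spline point down, placing it just above the hit surface.
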(event Custom|Snap%20to%20Ground
  ;[1 1 1] Snap Spline to Ground
  (for _index (range 0 (Spline|GetNumberOfSplinePoints (Variables|Default|GetSpline)))
    (bind _output_get (Variables|Default|SetCurrent%20index _index))
    (bind (_outhit _returnvalue) (Collision|LineTraceByChannel (Spline|GetLocationatSplinePoint (Variables|Default|GetSpline) _output_get "World") (+ (Spline|GetLocationatSplinePoint (Variables|Default|GetSpline) _output_get "World") (* "0.000000,0.000000,-1.000000" (Variables|Default|GetGround%20Trace%20Distance))) "TraceTypeQuery1" false 0 "None"))
    (if _returnvalue
      (Spline|SetLocationatSplinePoint (Variables|Default|GetSpline) (Variables|Default|GetCurrent%20index) (+ (.Location (Collision|BreakHitResult _outhit)) "0.000000,0.000000,20.000000") "World" true))))

(event Custom|Spawn%20Pedestrians
  (bind _spline (Variables|Default|GetSpline))
  (bind _spline_2 (Variables|Default|GetSpline))
  (bind _returnvalue (Spline|GetSplineLength _spline))
  (bind _returnvalue_2 (/ _returnvalue 1.2))
  (bind _returnvalue_3 (/ _returnvalue 3.0))
  (bind _returnvalue_4 (Math|Random|RandomFloatinRange _returnvalue_3 _returnvalue_2))
  (bind _returnvalue_5 (Spline|GetTransformatDistanceAlongSpline _spline_2 _returnvalue_4 "World" false))
  ;[1 1 1] Spawn Pedestrians
  (if (Variables|Default|GetSpawn%20Pedestrians?)
    (Utilities|FlowControl|Delay 1.0)
    (if (> (Variables|Default|GetNumber%20of%20pedestrians%20to%20spawn) 0)
      (Variables|Default|SetNumber%20of%20pedestrians%20to%20spawn (- (Variables|Default|GetNumber%20of%20pedestrians%20to%20spawn) 1))
      (bind _returnvalue_6 (AI|SpawnAIFromClass "/Game/IntelligentTrafficSystem/Blueprints/Pedestrian_BPs/BP_Pedestrian.BP_Pedestrian_C" "/Game/IntelligentTrafficSystem/Blueprints/Pedestrian_BPs/BT_Pedestrian.BT_Pedestrian" (.location _returnvalue_5) (.rotation _returnvalue_5) true 0))
      (bind _asbp_pedestrian (Utilities|Casting|CastToBP_Pedestrian _returnvalue_6))
      (Utilities|IsValid _asbp_pedestrian
        (:Is%20Valid
          (Variables|/Game/IntelligentTrafficSystem/Blueprints/Pedestrian_BPs/BP_Pedestrian.BP_Pedestrian_C|SetActive%20Path _asbp_pedestrian self)
          (CallFunction|SpawnPedestrians))))))

(event EventBeginPlay
  (CallFunction|SpawnPedestrians))

(event Collision|EventActorBeginOverlap
  (params (OtherActor :type Actor%20Object%20Reference)))

(fn ConstructionScript)