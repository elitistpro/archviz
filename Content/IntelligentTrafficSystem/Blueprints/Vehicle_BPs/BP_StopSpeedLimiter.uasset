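; BP_StopSpeedLimiter is a trigger box for the traffic system that makes AI cars pause and changes their speed limits.
; When a BP_Ai_car enters, it receives the box's max and min speeds, and its Blackboard "Stop" key and StopForSpeedLimiter flag are set.
; After a random Delay between the configured wait times, the stop is cleared.
; A single Delay serves all overlaps, so cars entering during a wait get no release of their own.
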(event OnComponentBeginOverlap(Box)
  (params (OverlappedComponent :type Primitive%20Component%20Object%20Reference) (OtherActor :type Actor%20Object%20Reference) (OtherComp :type Primitive%20Component%20Object%20Reference) (OtherBodyIndex :type Integer) (bFromSweep :type Boolean) (SweepResult :type Hit%20Result%20Structure%20%28by%20ref%29))
  (bind _returnvalue (Utilities|Name|MakeLiteralName "Stop"))
  (bind _asbp_ai_car (Utilities|Casting|CastToBP_Ai_car OtherActor))
  (Variables|Default|Setai%20car%20ref _asbp_ai_car)
  (Variables|/Game/IntelligentTrafficSystem/Blueprints/Vehicle_BPs/BP_Ai_car.BP_Ai_car_C|SetMax%20Speed _asbp_ai_car (Variables|Default|GetMax%20Speed))
  (Variables|/Game/IntelligentTrafficSystem/Blueprints/Vehicle_BPs/BP_Ai_car.BP_Ai_car_C|SetMin%20Speed _asbp_ai_car (Variables|Default|GetMin%20Speed))
  (AI|Components|Blackboard|SetValueasBool (AI|GetBlackboard _asbp_ai_car) _returnvalue true)
  (Variables|/Game/IntelligentTrafficSystem/Blueprints/Vehicle_BPs/BP_Ai_car.BP_Ai_car_C|SetStop%20for%20speed%20limiter _asbp_ai_car true)
  (Utilities|FlowControl|Delay (Math|Random|RandomFloatinRange (Variables|Default|GetMin%20wait%20time) (Variables|Default|GetMax%20wait%20time)))
  (Utilities|IsValid _asbp_ai_car
    (:Is%20Valid
      (Variables|/Game/IntelligentTrafficSystem/Blueprints/Vehicle_BPs/BP_Ai_car.BP_Ai_car_C|SetStop%20for%20speed%20limiter _asbp_ai_car false))
    (:Is%20Not%20Valid
      (bind _output_get (Variables|Default|Setai%20car%20ref 0))
      (Variables|/Game/IntelligentTrafficSystem/Blueprints/Vehicle_BPs/BP_Ai_car.BP_Ai_car_C|SetStop%20for%20speed%20limiter _output_get false)))
  (AI|Components|Blackboard|SetValueasBool (AI|GetBlackboard _asbp_ai_car) _returnvalue false))

(event EventBeginPlay)

(event Collision|EventActorBeginOverlap
  (params (OtherActor :type Actor%20Object%20Reference)))

(event EventTick
  (params (DeltaSeconds :type Float%20%28single-precision%29)))

(fn ConstructionScript)