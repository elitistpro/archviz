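; BP_TrafficLight is a traffic light that controls AI cars in the traffic system.
; From its starting color it loops green, yellow, red and red-yellow on delays, toggling light visibility and setting a Stop flag for all but green.
; Its trigger box writes Stop to overlapping non-service cars' Blackboards, rechecking via a retriggerable delay on the last stored car.
; Green also clears the car-close-ahead key, and leaving the box clears Stop.
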(event OnComponentBeginOverlap(Box)
  (params (OverlappedComponent :type Primitive%20Component%20Object%20Reference) (OtherActor :type Actor%20Object%20Reference) (OtherComp :type Primitive%20Component%20Object%20Reference) (OtherBodyIndex :type Integer) (bFromSweep :type Boolean) (SweepResult :type Hit%20Result%20Structure%20%28by%20ref%29))
  ;[1 1 1] Controlling TraFFIC
  (bind _asbp_ai_car (Utilities|Casting|CastToBP_Ai_car OtherActor))
  (bind _output_get (Variables|Default|SetAs%20BP%20Ai%20Car _asbp_ai_car))
  (if (not (Variables|/Game/IntelligentTrafficSystem/Blueprints/Vehicle_BPs/BP_Ai_car.BP_Ai_car_C|GetService%20Car _output_get))
    (if (Variables|Default|GetStop) :!label _label
      (Utilities|IsValid (AI|GetBlackboard _output_get)
        (:Is%20Valid
          (AI|Components|Blackboard|SetValueasBool (AI|GetBlackboard _output_get) (Utilities|Name|MakeLiteralName "Stop") true)
          (Utilities|FlowControl|RetriggerableDelay 3.0)
          (goto _label)))
      (else
        (Utilities|IsValid (AI|GetBlackboard _output_get)
          (:Is%20Valid
            (AI|Components|Blackboard|SetValueasBool (AI|GetBlackboard _output_get) (Utilities|Name|MakeLiteralName "Stop") false)
            (AI|Components|Blackboard|SetValueasBool (AI|GetBlackboard _output_get) (Utilities|Name|MakeLiteralName "car close ahead") false)))))))

(event OnComponentEndOverlap(Box)
  (params (OverlappedComponent :type Primitive%20Component%20Object%20Reference) (OtherActor :type Actor%20Object%20Reference) (OtherComp :type Primitive%20Component%20Object%20Reference) (OtherBodyIndex :type Integer))
  (bind _asbp_ai_car (Utilities|Casting|CastToBP_Ai_car OtherActor))
  (Utilities|IsValid (AI|GetBlackboard _asbp_ai_car)
    (:Is%20Valid
      (AI|Components|Blackboard|SetValueasBool (AI|GetBlackboard _asbp_ai_car) (Utilities|Name|MakeLiteralName "Stop") false))))

(event Custom|Set%20Traffic%20light%20colour
  (params (Traffic%20light%20color :type E_TrafficLightColorEnum%20Enum :default "NewEnumerator0"))
  ;[1 1 1] Light Change
  (bind _output_get (Variables|Default|SetTraffic%20light%20colors Traffic%20light%20color))
  (switch Utilities|FlowControl|Switch|SwitchonE_TrafficLightColorEnum _output_get
    (:NewEnumerator0
      (Variables|Default|SetStop false)
      (CallFunction|ToggleGreenLight true)
      (CallFunction|ToggleYellowLight false)
      (CallFunction|ToggleRedLight false)
      (Utilities|FlowControl|Delay (Variables|Default|GetGreen%20light%20Duration))
      (CallFunction|SetTrafficLightColour "NewEnumerator1"))
    (:NewEnumerator1
      (Variables|Default|SetStop true)
      (CallFunction|ToggleYellowLight true)
      (CallFunction|ToggleGreenLight false)
      (Utilities|FlowControl|Delay 3.0)
      (CallFunction|SetTrafficLightColour "NewEnumerator2"))
    (:NewEnumerator2
      (Variables|Default|SetStop true)
      (CallFunction|ToggleRedLight true)
      (CallFunction|ToggleYellowLight false)
      (Utilities|FlowControl|Delay (Variables|Default|GetRed%20light%20Duration))
      (CallFunction|SetTrafficLightColour "NewEnumerator3"))
    (:NewEnumerator3
      (Variables|Default|SetStop true)
      (CallFunction|ToggleYellowLight true)
      (Utilities|FlowControl|Delay 2.0)
      (CallFunction|SetTrafficLightColour "NewEnumerator0"))))

(event EventBeginPlay
  ;[1 1 1] Initiate traffic light color
  (CallFunction|SetTrafficLightColour (Variables|Default|GetStarting%20color)))

(fn ConstructionScript)

(fn ToggleGreenLight
  (params (On? :type Boolean))
  (Rendering|SetVisibility (Variables|Default|GetGreen%20light) On? false))

(fn ToggleYellowLight
  (params (On? :type Boolean))
  (Rendering|SetVisibility (Variables|Default|GetYellow%20light) On? false))

(fn ToggleRedLight
  (params (On? :type Boolean))
  (Rendering|SetVisibility (Variables|Default|GetRed%20light) On? false))