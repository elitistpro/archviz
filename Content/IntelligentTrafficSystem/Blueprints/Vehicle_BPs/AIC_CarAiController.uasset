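; AI controller for BP_Ai_car traffic and race cars that runs the BT_AiCAr behavior tree and sizes pawn sensing by car type.
; A self-recalling, delayed avoidance loop brakes traffic cars near obstacles, while racers brake and switch to a random linked lane path.
; The sight-based obstruction logic that writes blackboard keys is disconnected from OnSeePawn.
; VehicleCounter is a looping debug car count, uncalled here.
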(event OnSeePawn(PawnSensing)
  (params (Pawn :type Pawn%20Object%20Reference)))

(event Custom|Collision%20avoidance
  ;[1 1 1] Collision avlidance
  (if (Variables|Default|GetChanging%20lanes)
    (Utilities|FlowControl|Delay 1.0)
    (Variables|Default|SetChanging%20lanes false)
    (CallFunction|CollisionAvoidance)
    (else
      (Utilities|FlowControl|Delay 0.2)
      (bind _asbp_ai_car (Utilities|Casting|CastToBP_Ai_car (Pawn|GetControlledPawn)))
      (if (Variables|/Game/IntelligentTrafficSystem/Blueprints/Vehicle_BPs/BP_Ai_car.BP_Ai_car_C|GetRacing? _asbp_ai_car)
        (if (Variables|/Game/IntelligentTrafficSystem/Blueprints/Vehicle_BPs/BP_Ai_car.BP_Ai_car_C|GetCollision%20avoidance _asbp_ai_car)
          (Class|ChaosVehicleMovementComponent|SetBrakeInput (Variables|/Script/ChaosVehicles.WheeledVehiclePawn|GetVehicleMovementComponent _asbp_ai_car) 1.0)
          (Variables|Default|SetChanging%20lanes true)
          (Variables|/Game/IntelligentTrafficSystem/Blueprints/Vehicle_BPs/BP_Ai_car.BP_Ai_car_C|SetActivePath _asbp_ai_car (.OutItem (Utilities|Array|Random (Variables|/Game/IntelligentTrafficSystem/Blueprints/Vehicle_BPs/BP_Path.BP_Path_C|GetLanes%20To%20change%20to (Variables|/Game/IntelligentTrafficSystem/Blueprints/Vehicle_BPs/BP_Ai_car.BP_Ai_car_C|GetActivePath _asbp_ai_car)))))
          (CallFunction|CollisionAvoidance)
          (else
            (CallFunction|CollisionAvoidance)))
        (elif (< (Variables|/Game/IntelligentTrafficSystem/Blueprints/Vehicle_BPs/BP_Ai_car.BP_Ai_car_C|GetOut%20Hit%20Distance _asbp_ai_car) 5e+02)
          (Class|ChaosVehicleMovementComponent|SetBrakeInput (Variables|/Script/ChaosVehicles.WheeledVehiclePawn|GetVehicleMovementComponent _asbp_ai_car) 1.0)
          (CallFunction|CollisionAvoidance)
          (else
            (CallFunction|CollisionAvoidance)))))))

(event Custom|Vehicle%20Counter
  (Utilities|FlowControl|Delay 0.5)
  (bind _outactors (Actor|GetAllActorsOfClass "/Game/IntelligentTrafficSystem/Blueprints/Vehicle_BPs/BP_Ai_car.BP_Ai_car_C"))
  (Development|PrintString (Utilities|String|ToString(Integer) (Utilities|Array|Length _outactors)) true true "(R=0.000000,G=1.000000,B=0.143920,A=1.000000)" 0.6)
  (CallFunction|VehicleCounter))

(event EventBeginPlay
  (bind _pawnsensing (Variables|Default|GetPawnSensing))
  (bind _pawnsensing_2 (Variables|Default|GetPawnSensing))
  (Utilities|FlowControl|Sequence
    (:then_0
      (AI|RunBehaviorTree "/Game/IntelligentTrafficSystem/Blueprints/Vehicle_BPs/BT_AiCAr.BT_AiCAr"))
    (:then_1
      ;[1 1 1] Setting the pawn sensing radius for the traffic and race car
      (bind _asbp_ai_car (Utilities|Casting|CastToBP_Ai_car (Pawn|GetControlledPawn self)))
      (if (Variables|/Game/IntelligentTrafficSystem/Blueprints/Vehicle_BPs/BP_Ai_car.BP_Ai_car_C|GetRacing? _asbp_ai_car)
        (Variables|/Script/AIModule.PawnSensingComponent|SetSightRadius _pawnsensing 2.5e+03)
        (Class|PawnSensingComponent|SetPeripheralVisionAngle _pawnsensing 3e+01)
        (else
          (Variables|/Script/AIModule.PawnSensingComponent|SetSightRadius _pawnsensing_2 8e+02)
          (Class|PawnSensingComponent|SetPeripheralVisionAngle _pawnsensing_2 25.0))))
    (:then_2
      (CallFunction|CollisionAvoidance))))

(fn ConstructionScript)