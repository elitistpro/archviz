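; AI vehicle pawn for the Intelligent Traffic System, driving BP_Path splines as traffic or as a racer.
; Steering targets a point ahead on the spline, corrected by velocity-based path prediction.
; Line traces, pawn sensing and traffic-light overlaps set blackboard flags, while traffic obstructions also brake the car directly.
; Tick also runs stuck recovery, teleporting traffic to free parking and racers to their target; other events handle pedestrian ragdolls and day/night headlights.
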(event OnComponentBeginOverlap(Box)
  (params (OverlappedComponent :type Primitive%20Component%20Object%20Reference) (OtherActor :type Actor%20Object%20Reference) (OtherComp :type Primitive%20Component%20Object%20Reference) (OtherBodyIndex :type Integer) (bFromSweep :type Boolean) (SweepResult :type Hit%20Result%20Structure%20%28by%20ref%29))
  (bind _asbp_pedestrian (Utilities|Casting|CastToBP_Pedestrian OtherActor))
  (Default|Ragdoll _asbp_pedestrian self))

(event OnSeePawn(PawnSensing)
  (params (Pawn :type Pawn%20Object%20Reference))
  (if (!= Pawn (Variables|Default|GetBp%20Ai%20Cars))
    (AI|Components|Blackboard|SetValueasBool (AI|GetBlackboard 0) (Utilities|Name|MakeLiteralName "Pedestrian Ahead") true)
    (Utilities|FlowControl|RetriggerableDelay 1.0)
    (AI|Components|Blackboard|SetValueasBool (AI|GetBlackboard 0) (Utilities|Name|MakeLiteralName "Pedestrian Ahead") false)
    (else
      (AI|Components|Blackboard|SetValueasBool (AI|GetBlackboard 0) (Utilities|Name|MakeLiteralName "Pedestrian Ahead") false))))

(event Custom|Steer
  (bind _returnvalue (Transformation|GetActorLocation))
  (bind _returnvalue_2 (Transformation|GetActorLocation))
  (bind _activepath (Variables|Default|GetActivePath))
  (bind _activepath_2 (Variables|Default|GetActivePath))
  (bind _activepath_3 (Variables|Default|GetActivePath))
  (bind _path_spline (Variables|/Game/IntelligentTrafficSystem/Blueprints/Vehicle_BPs/BP_Path.BP_Path_C|GetPath%20Spline _activepath))
  (bind _path_spline_2 (Variables|/Game/IntelligentTrafficSystem/Blueprints/Vehicle_BPs/BP_Path.BP_Path_C|GetPath%20Spline _activepath_2))
  (Utilities|IsValid _activepath_3
    (:Is%20Valid
      (if (Variables|/Game/IntelligentTrafficSystem/Blueprints/Vehicle_BPs/BP_Path.BP_Path_C|GetRacing? _activepath_3)
        (Variables|Default|SetTarget%20point (Spline|FindLocationClosesttoWorldLocation _path_spline (+ (* (Math|Vector|Normalize (Class|SplineComponent|FindTangentClosesttoWorldLocation _path_spline _returnvalue "World")) (Variables|Default|GetRacing%20Target%20Point%20Distance)) _returnvalue) "World"))
        (else
          (Utilities|IsValid _path_spline_2
            (:Is%20Valid
              (Variables|Default|SetTarget%20point (Spline|FindLocationClosesttoWorldLocation _path_spline_2 (+ (* (Math|Vector|Normalize (Class|SplineComponent|FindTangentClosesttoWorldLocation _path_spline_2 _returnvalue_2 "World")) 6e+02) _returnvalue_2) "World"))))))
      (if (< (Math|Vector|Distance(Vector) (Variables|Default|GetTarget%20point) (Transformation|GetActorLocation)) (Variables|Default|GetCheckGap))
        (Variables|Default|SetTarget%20spline%20Distance (Math|Float|SelectFloat 0.0 (+ (Variables|Default|GetTarget%20spline%20Distance) (Variables|Default|GetDist%20Increment%20Gap)) (> (+ (Variables|Default|GetTarget%20spline%20Distance) (Variables|Default|GetDist%20Increment%20Gap)) (Spline|GetSplineLength (Variables|/Game/IntelligentTrafficSystem/Blueprints/Vehicle_BPs/BP_Path.BP_Path_C|GetPath%20Spline (Variables|Default|GetActivePath)))))))
      (bind _steering (CallFunction|PredictPath))
      (Class|ChaosVehicleMovementComponent|SetSteeringInput (Variables|Default|GetVehicleMovementComponent) _steering))))

(event Custom|Check%20lTraffic%20light%20color
  (bind _returnvalue (AI|GetBlackboard 0))
  (bind _overlappingactors (Collision|GetOverlappingActors "/Game/IntelligentTrafficSystem/Blueprints/Vehicle_BPs/BP_TrafficLight.BP_TrafficLight_C" :!class /Script/Engine.Actor))
  (bind _returnvalue_2 (Utilities|Name|MakeLiteralName "Stop"))
  ;[1 1 1] Check traffic light color
  (if (> (Utilities|Array|Length _overlappingactors) 0)
    (for _array_element _overlappingactors
      (bind _asbp_traffic_light (Utilities|Casting|CastToBP_TrafficLight _array_element))
      (if (Variables|/Game/IntelligentTrafficSystem/Blueprints/Vehicle_BPs/BP_TrafficLight.BP_TrafficLight_C|GetStop _asbp_traffic_light)
        (AI|Components|Blackboard|SetValueasBool _returnvalue _returnvalue_2 true)
        (else
          (AI|Components|Blackboard|SetValueasBool _returnvalue _returnvalue_2 false))))))

(event Custom|Fix%20stuck%20cars
  (bind _current_speed (Variables|Default|GetCurrent%20speed))
  (bind _unoccupied_parking_spots (Variables|Default|GetUnoccupied%20parking%20spots))
  (bind _outitem (Utilities|Array|Random _unoccupied_parking_spots))
  ;[1 1 1] Fix stuck cars
  (if (and (< _current_speed 2.0) (> _current_speed -2.0))
    (if (< (Variables|Default|GetDespawnTimer) 1.0)
      (if (Variables|Default|GetRacing?)
        (Transformation|Teleport self (Variables|Default|GetTarget%20point) "0, 0, 0")
        (else
          (bind _outactors (Actor|GetAllActorsOfClass "/Game/IntelligentTrafficSystem/Blueprints/Vehicle_BPs/BP_Path.BP_Path_C"))
          (for _array_element _outactors
            (if (Variables|/Game/IntelligentTrafficSystem/Blueprints/Vehicle_BPs/BP_Path.BP_Path_C|GetParking _array_element)
              (if (not (Variables|/Game/IntelligentTrafficSystem/Blueprints/Vehicle_BPs/BP_Path.BP_Path_C|GetIs%20Occupied? _array_element))
                (Utilities|Array|Add _unoccupied_parking_spots _array_element))))
          (Utilities|IsValid _outitem
            (:Is%20Valid
              (bind _output_get (Variables|Default|SetActivePath _outitem))
              (Variables|/Game/IntelligentTrafficSystem/Blueprints/Vehicle_BPs/BP_Path.BP_Path_C|SetIs%20Occupied? _output_get true)
              (bind _returnvalue (Transformation|Teleport self (+ (Spline|GetLocationatSplinePoint (Variables|/Game/IntelligentTrafficSystem/Blueprints/Vehicle_BPs/BP_Path.BP_Path_C|GetPath%20Spline _output_get) 0 "World") "0.000000,0.000000,50.000000") (Spline|GetRotationatSplinePoint (Variables|/Game/IntelligentTrafficSystem/Blueprints/Vehicle_BPs/BP_Path.BP_Path_C|GetPath%20Spline _output_get) 0 "World")))
              (if _returnvalue
                (Variables|Default|SetGoing%20through%20intersection false)
                (Variables|Default|SetIntersection%20timestamp 0)
                (Utilities|Array|Clear (Variables|Default|GetUnoccupied%20parking%20spots))
                (AI|Components|Blackboard|SetValueasBool (AI|GetBlackboard 0) (Utilities|Name|MakeLiteralName "Intersection Blocked?") false)
                (Variables|Default|SetDespawnTimer 1e+01)
                (Default|ResetOccupiedStatusAfterParking _output_get))))))
      (elif (ScalableFloat|GetValueasBool (AI|GetBlackboard self) (Utilities|Name|MakeLiteralName "Stop"))
        (Variables|Default|SetDespawnTimer 1e+01 :!label _label)
        (elif (Variables|Default|GetParked)
          (goto _label)
          (elif (Variables|Default|GetStop%20for%20speed%20limiter)
            (goto _label)
            (else
              (Utilities|FlowControl|Delay 1.0)
              (Variables|Default|SetDespawnTimer (- (Variables|Default|GetDespawnTimer) 1.0)))))))
    (else
      (Variables|Default|SetDespawnTimer 1e+01))))

(event Custom|Debug%20brake%20input
  (bind _vehiclemovementcomponent (Variables|Default|GetVehicleMovementComponent))
  ;[1 1 1] Debug brake input
  (if (not (Variables|Default|GetRacing?))
    (bind _returnvalue (Class|ChaosVehicleMovementComponent|GetBrakeInput _vehiclemovementcomponent))
    (Development|PrintString (Utilities|String|ToString(Float) _returnvalue))
    (if (Class|ChaosVehicleMovementComponent|GetHandbrakeInput _vehiclemovementcomponent)
      (Development|PrintString "Handbrake on"))))

(event Custom|Intersection%20priority%20timestamp
  ;[1 1 1] Intersection timestamp
  (Utilities|FlowControl|Delay 1.0)
  (if (Variables|Default|GetGoing%20through%20intersection)
    (Variables|Default|SetIntersection%20timestamp (+ (Variables|Default|GetIntersection%20timestamp) 1))))

(event Custom|Park%20stuck%20car
  (bind _unoccupied_parking_spots (Variables|Default|GetUnoccupied%20parking%20spots))
  (bind _outitem (Utilities|Array|Random _unoccupied_parking_spots))
  ;[1 1 1] Fix stuck cars
  (bind _outactors (Actor|GetAllActorsOfClass "/Game/IntelligentTrafficSystem/Blueprints/Vehicle_BPs/BP_Path.BP_Path_C"))
  (for _array_element _outactors
    (if (Variables|/Game/IntelligentTrafficSystem/Blueprints/Vehicle_BPs/BP_Path.BP_Path_C|GetParking _array_element)
      (if (not (Variables|/Game/IntelligentTrafficSystem/Blueprints/Vehicle_BPs/BP_Path.BP_Path_C|GetIs%20Occupied? _array_element))
        (Utilities|Array|Add _unoccupied_parking_spots _array_element))))
  (Utilities|IsValid _outitem
    (:Is%20Valid
      (bind _output_get (Variables|Default|SetActivePath _outitem))
      (Variables|/Game/IntelligentTrafficSystem/Blueprints/Vehicle_BPs/BP_Path.BP_Path_C|SetIs%20Occupied? _output_get true)
      (bind _returnvalue (Transformation|Teleport self (+ (Spline|GetLocationatSplinePoint (Variables|/Game/IntelligentTrafficSystem/Blueprints/Vehicle_BPs/BP_Path.BP_Path_C|GetPath%20Spline _output_get) 0 "World") "0.000000,0.000000,50.000000") (Spline|GetRotationatSplinePoint (Variables|/Game/IntelligentTrafficSystem/Blueprints/Vehicle_BPs/BP_Path.BP_Path_C|GetPath%20Spline _output_get) 0 "World")))
      (if _returnvalue
        (Variables|Default|SetGoing%20through%20intersection false)
        (Variables|Default|SetIntersection%20timestamp 0)
        (Utilities|Array|Clear (Variables|Default|GetUnoccupied%20parking%20spots))
        (AI|Components|Blackboard|SetValueasBool (AI|GetBlackboard 0) (Utilities|Name|MakeLiteralName "Intersection Blocked?") false)
        (Variables|Default|SetDespawnTimer 1e+01)
        (Default|ResetOccupiedStatusAfterParking _output_get)))))

(event Custom|Despawn%20Vehicle
  (bind _returnvalue (Game|GetPlayerCharacter 0))
  (bind _initial_path (Variables|Default|GetInitial%20Path))
  ;[1 1 1] Despawn Vehicles
  (Utilities|IsValid _returnvalue
    (:Is%20Valid
      (if (not (< (Math|Vector|Distance(Vector) (Transformation|GetActorLocation _returnvalue) (Transformation|GetActorLocation self)) 1.4e+04))
        (if (< (Variables|/Game/IntelligentTrafficSystem/Blueprints/Vehicle_BPs/BP_Path.BP_Path_C|GetNumber%20of%20cars%20to%20spawn _initial_path) 1)
          (Variables|/Game/IntelligentTrafficSystem/Blueprints/Vehicle_BPs/BP_Path.BP_Path_C|SetNumber%20of%20cars%20to%20spawn _initial_path (+ (Variables|/Game/IntelligentTrafficSystem/Blueprints/Vehicle_BPs/BP_Path.BP_Path_C|GetNumber%20of%20cars%20to%20spawn _initial_path) 1))
          (Actor|DestroyActor)
          (else
            (Actor|DestroyActor)))))))

(event EventTick
  (params (DeltaSeconds :type Float%20%28single-precision%29))
  (bind _returnvalue (Utilities|Name|MakeLiteralName "Intersection Blocked?"))
  (bind _returnvalue_2 (AI|GetBlackboard 0))
  (bind _returnvalue_3 (Utilities|Name|MakeLiteralName "Car Hit"))
  (bind _returnvalue_4 (Utilities|Name|MakeLiteralName "Car Hit"))
  (Utilities|FlowControl|Sequence
    (:then_0
      ;[1 1 1] Event Tick
      (Utilities|FlowControl|Delay 0.5)
      (CallFunction|CheckLTrafficLightColor))
    (:then_1
      (Utilities|FlowControl|Delay 3.0)
      (Variables|Default|SetChanging%20Lanes? false)
      (Variables|Default|SetRacing%20Target%20Point%20Distance 2e+03))
    (:then_2
      (Variables|Default|SetCurrent%20speed (* (Class|ChaosVehicleMovementComponent|GetForwardSpeedMPH (Variables|Default|GetVehicleMovementComponent)) 1.609)))
    (:then_3
      (Utilities|FlowControl|Delay 1.0)
      (CallFunction|FixStuckCars))
    (:then_4
      ;;[1 1 1] Speed limiter fix
      (Utilities|FlowControl|Delay 3.0)
      (if (Variables|Default|GetStop%20for%20speed%20limiter)
        (if (== (Utilities|Array|Length (Collision|GetOverlappingActors self "/Game/IntelligentTrafficSystem/Blueprints/Vehicle_BPs/BP_StopSpeedLimiter.BP_StopSpeedLimiter_C" :!class /Script/Engine.Actor)) 0)
          (Variables|Default|SetStop%20for%20speed%20limiter false))))
    (:then_5
      ;;[1 1 1] Fix for brakes not working when exiting parking
      (bind _returnvalue_5 (Class|ChaosVehicleMovementComponent|GetBrakeInput (Variables|Default|GetVehicleMovementComponent)))
      (if (and (ScalableFloat|GetValueasBool (AI|GetBlackboard 0) (Utilities|Name|MakeLiteralName "Exit parking?")) (> _returnvalue_5 0.0))
        (Class|ChaosVehicleMovementComponent|SetBrakeInput (Variables|Default|GetVehicleMovementComponent) 0.0)))
    (:then_6
      (if (Variables|Default|GetGoing%20through%20intersection)
        (if (not (ScalableFloat|GetValueasBool (AI|GetBlackboard 0) (Utilities|Name|MakeLiteralName "Exit parking?")))
          (Utilities|FlowControl|Sequence
            (:then_0
              (bind (_outhit _returnvalue_6) (Collision|LineTraceByChannel (Transformation|GetWorldLocation (Variables|Default|GetLook%20left)) (Transformation|GetWorldLocation (Variables|Default|GetLook%20left%20End)) "TraceTypeQuery1" false 0 "None"))
              (bind _asbp_ai_car (Utilities|Casting|CastToBP_Ai_car (.hitactor _outhit)))
              (bind _output_get (Variables|Default|SetIntersection%20obstructing%20car _asbp_ai_car))
              (bind _output_get_2 (Variables|Default|SetIntersection%20out%20hit%20distance (.distance _outhit)))
              (Variables|Default|SetIntersection%20Left%20Blocked _returnvalue_6)
              (if (< _output_get_2 2e+02)
                (AI|Components|Blackboard|SetValueasBool (AI|GetBlackboard 0) (Utilities|Name|MakeLiteralName "Car Hit") true)
                (Utilities|FlowControl|RetriggerableDelay 0.5)
                (Variables|Default|SetIntersection%20obstructing%20car 0)
                (else
                  (AI|Components|Blackboard|SetValueasBool (AI|GetBlackboard 0) _returnvalue_3 false)
                  (AI|Components|Blackboard|SetValueasBool (AI|GetBlackboard _output_get) _returnvalue_3 false)
                  (Utilities|FlowControl|RetriggerableDelay 0.5)
                  (Variables|Default|SetIntersection%20obstructing%20car 0)))
              (AI|Components|Blackboard|SetValueasBool (AI|GetBlackboard 0) (Utilities|Name|MakeLiteralName "Car Hit") false)
              (Variables|Default|SetIntersection%20Right%20Blocked false))
            (:then_1
              (bind (_outhit_2 _returnvalue_7) (Collision|LineTraceByChannel (Transformation|GetWorldLocation (Variables|Default|GetLook%20right)) (Transformation|GetWorldLocation (Variables|Default|GetLook%20right%20End)) "TraceTypeQuery1" false 0 "None"))
              (bind _asbp_ai_car_2 (Utilities|Casting|CastToBP_Ai_car (.hitactor _outhit_2)))
              (bind _output_get_3 (Variables|Default|SetIntersection%20obstructing%20car _asbp_ai_car_2))
              (bind _output_get_4 (Variables|Default|SetIntersection%20out%20hit%20distance (.distance _outhit_2)))
              (Variables|Default|SetIntersection%20Right%20Blocked _returnvalue_7)
              (if (< _output_get_4 2e+02)
                (AI|Components|Blackboard|SetValueasBool (AI|GetBlackboard 0) (Utilities|Name|MakeLiteralName "Car Hit") true)
                (Utilities|FlowControl|RetriggerableDelay 0.5)
                (Variables|Default|SetIntersection%20obstructing%20car 0)
                (else
                  (AI|Components|Blackboard|SetValueasBool (AI|GetBlackboard 0) _returnvalue_4 false)
                  (AI|Components|Blackboard|SetValueasBool (AI|GetBlackboard _output_get_3) _returnvalue_4 false)
                  (Utilities|FlowControl|RetriggerableDelay 0.5)
                  (Variables|Default|SetIntersection%20obstructing%20car 0)))
              (AI|Components|Blackboard|SetValueasBool (AI|GetBlackboard 0) (Utilities|Name|MakeLiteralName "Car Hit") false)
              (Variables|Default|SetIntersection%20Right%20Blocked false))))
        (else
          (AI|Components|Blackboard|SetValueasBool (AI|GetBlackboard 0) (Utilities|Name|MakeLiteralName "Intersection Blocked?") false))))
    (:then_7
      (Utilities|IsValid (Variables|Default|GetIntersection%20obstructing%20car)
        (:Is%20Valid
          (if (Variables|Default|GetGoing%20through%20intersection)
            (if (Variables|Default|GetIntersection%20Right%20Blocked)
              (if (Variables|Default|GetIntersection%20Left%20Blocked)
                (AI|Components|Blackboard|SetValueasBool _returnvalue_2 _returnvalue true)
                (else
                  (AI|Components|Blackboard|SetValueasBool _returnvalue_2 _returnvalue true)))
              (elif (Variables|Default|GetIntersection%20Left%20Blocked)
                (AI|Components|Blackboard|SetValueasBool _returnvalue_2 _returnvalue true)
                (else
                  (AI|Components|Blackboard|SetValueasBool _returnvalue_2 _returnvalue false :!label _label)
                  (AI|Components|Blackboard|SetValueasBool (AI|GetBlackboard 0) (Utilities|Name|MakeLiteralName "Car Hit") false))))
            (else
              (goto _label))))
        (:Is%20Not%20Valid
          (goto _label))))
    (:then_9
      (CallFunction|IntersectionPriorityTimestamp))))

(event EventBeginPlay
  (Utilities|FlowControl|Sequence
    (:then_0
      (Components|SkeletalMesh|SetSkeletalMeshAsset (Variables|Character|GetMesh) (.OutItem (Utilities|Array|Random (Variables|Default|GetVehicle%20Mesh)))))
    (:then_1
      ;[1 1 1] Fix Random invisible Collisions
      (Variables|/Script/Engine.SkinnedMeshComponent|SetVisibilityBasedAnimTickOption (Variables|Character|GetMesh) "AlwaysTickPoseAndRefreshBones")
      (CallFunction|Headlights 0.0))))

(event EventDayShift
  (CallFunction|Headlights 0.0))

(event EventNightShift
  (CallFunction|Headlights 1.0))

(fn ConstructionScript)

(fn BrakeLights
  (params (BrakeLights :type Boolean))
  (bind _returnvalue (Rendering|Material|CreateDynamicMaterialInstance "/Game/IntelligentTrafficSystem/Demo/SportsCar/Materials/MI_SportsCar_Chassis.MI_SportsCar_Chassis" "" "None" :!class /Script/Engine.KismetMaterialLibrary))
  (Rendering|Material|SetMaterial (Variables|Character|GetMesh) 0 _returnvalue)
  (if BrakeLights
    (Rendering|Material|SetScalarParameterValue _returnvalue "BrakeLightPower" 2e+02 :!class /Script/Engine.MaterialInstanceDynamic)
    (else
      (Rendering|Material|SetScalarParameterValue _returnvalue "BrakeLightPower" 4.0 :!class /Script/Engine.MaterialInstanceDynamic))))

(fn GetPath
  (Variables|Default|SetActive%20Path%20name (Utilities|GetObjectName (Variables|Default|GetActivePath)))
  (if (not (Variables|Default|GetChanging%20Lanes?))
    (CallFunction|Steer)))

(fn PredictPath
  (bind _returnvalue (Transformation|GetActorLocation))
  (bind _returnvalue_2 (Transformation|GetActorLocation))
  (bind _returnvalue_3 (Transformation|GetActorLocation))
  (bind _activepath (Variables|Default|GetActivePath))
  (bind _vehiclemovementcomponent (Variables|Default|GetVehicleMovementComponent))
  (bind _path_spline (Variables|/Game/IntelligentTrafficSystem/Blueprints/Vehicle_BPs/BP_Path.BP_Path_C|GetPath%20Spline _activepath))
  (Variables|Default|SetPredicted%20location _returnvalue)
  (Variables|Default|SetVelocity (Transformation|GetVelocity))
  (Variables|Default|SetTimestep (/ (/ (Math|Vector|Distance(Vector) _returnvalue (Variables|Default|GetTarget%20point)) (Math|Vector|VectorLength (Variables|Default|GetVelocity))) 5.0))
  (Variables|Default|SetSteer%20Yaw (.yaw (Math|Rotator|Delta(Rotator) (Math|Conversions|RotationFromXVector (Math|Vector|Normalize (Variables|Default|GetVelocity))) (Transformation|GetActorRotation))))
  (for _index (range 0 3)
    (Variables|Default|SetPredicted%20location (+ (Variables|Default|GetPredicted%20location) (* (Variables|Default|GetVelocity) (Variables|Default|GetTimestep))))
    (Variables|Default|SetVelocity (Math|Vector|RotateVectorAroundAxis (Variables|Default|GetVelocity) (Variables|Default|GetSteer%20Yaw) "0.000000,0.000000,1.000000")))
  (if (Variables|/Game/IntelligentTrafficSystem/Blueprints/Vehicle_BPs/BP_Path.BP_Path_C|GetRacing? (Variables|Default|GetActivePath))
    (bind _returnvalue_4 (Collision|LineTraceByChannel (Transformation|GetWorldLocation (Variables|Default|GetFront)) (+ (Spline|FindLocationClosesttoWorldLocation _path_spline (+ (* (Math|Vector|Normalize (Class|SplineComponent|FindTangentClosesttoWorldLocation _path_spline _returnvalue_3 "World")) 2.5e+03) _returnvalue_3) "World") "0.000000,0.000000,150.000000") "TraceTypeQuery1" false 0 "None" true "(R=0.054582,G=0.000000,B=1.000000,A=1.000000)" "(R=0.917504,G=0.938128,B=1.000000,A=1.000000)" 0.5))
    (Variables|Default|SetOut%20Hit%20Distance 0.0)
    (Variables|Default|SetObstruction%20ahead _returnvalue_4)
    (Variables|Default|SetCollision%20avoidance _returnvalue_4)
    (elif (Variables|Default|GetGoing%20through%20intersection)
      (AI|Components|Blackboard|SetValueasBool (AI|GetBlackboard 0) (Utilities|Name|MakeLiteralName "car close ahead") false)
      (else
        (bind (_outhit _returnvalue_5) (Collision|LineTraceByChannel (Transformation|GetWorldLocation (Variables|Default|GetFront)) (|Calculatetargetpoint) "TraceTypeQuery1" false 0 "None" true "(R=0.054582,G=0.000000,B=1.000000,A=1.000000)" "(R=0.917504,G=0.938128,B=1.000000,A=1.000000)" 0.2))
        (Variables|Default|SetObstructing%20actor (.hitactor _outhit))
        (bind _output_get (Variables|Default|SetOut%20Hit%20Distance (.distance _outhit)))
        (if (< _output_get (Variables|Default|GetTraffic%20target%20point%20distance))
          (bind _output_get_2 (Variables|Default|SetObstruction%20ahead _returnvalue_5))
          (bind _output_get_3 (Variables|Default|SetCollision%20avoidance _output_get_2))
          (if _output_get_3
            (CallFunction|RearLights 1.0)
            (AI|Components|Blackboard|SetValueasBool (AI|GetBlackboard 0) (Utilities|Name|MakeLiteralName "car close ahead") true :!label _label)
            (Class|ChaosVehicleMovementComponent|SetThrottleInput _vehiclemovementcomponent 0.0)
            (Class|ChaosVehicleMovementComponent|SetBrakeInput _vehiclemovementcomponent 1.0)
            (Class|ChaosVehicleMovementComponent|SetHandbrakeInput _vehiclemovementcomponent true)
            (else
              (bind _asaic_car_ai_controller (Utilities|Casting|CastToAIC_CarAiController (Pawn|GetController) :!label _label_2))
              (if (Variables|/Game/IntelligentTrafficSystem/Blueprints/Vehicle_BPs/AIC_CarAiController.AIC_CarAiController_C|GetObstruction%20Ahead? _asaic_car_ai_controller)
                (goto _label)
                (else
                  (CallFunction|RearLights 0.0)
                  (AI|Components|Blackboard|SetValueasBool (AI|GetBlackboard 0) (Utilities|Name|MakeLiteralName "car close ahead") false)))))
          (else
            (goto _label_2))))))
  (if (not (Math|Boolean|ORBoolean (Variables|Default|GetParked) (Variables|Default|GetStop) (ScalableFloat|GetValueasBool (AI|GetBlackboard 0) (Utilities|Name|MakeLiteralName "Exit parking?"))))
    (bind _output_get_4 (Variables|Default|SetSteering (* (.yaw (Math|Rotator|Delta(Rotator) (Math|Rotator|FindLookatRotation _returnvalue_2 (Variables|Default|GetPredicted%20location)) (Math|Rotator|FindLookatRotation _returnvalue_2 (Variables|Default|GetTarget%20point)))) -0.1)))
    (bind _output_get_5 (Variables|Default|Setcurrent%20steerimg (Math|Interpolation|FInterpTo (Variables|Default|Getcurrent%20steerimg) (Math|Float|Clamp(Float) _output_get_4 -1.0) (Utilities|Time|GetWorldDeltaSeconds) 4.0)))
    (return _output_get_5)))

(fn Headlights
  (params (Headlight%20Intensity :type Float%20%28single-precision%29))
  (Rendering|Material|SetScalarParameterValueonMaterials (Variables|Character|GetMesh) "Headlights" Headlight%20Intensity)
  (Rendering|Components|Light|SetIntensity (Variables|Default|GetLeft%20Headlight) (* Headlight%20Intensity 1e+05)))

(fn RearLights
  (params (Intensity :type Float%20%28single-precision%29))
  (Rendering|Material|SetScalarParameterValueonMaterials (Variables|Character|GetMesh) "Rear Lights" Intensity))

(fn AmbulanceLights
  (Utilities|FlowControl|FlipFlop
    (:A
      (CallFunction|RearLights 0.0)
      (CallFunction|Headlights 0.0))
    (:B
      (CallFunction|Headlights 1.0)
      (CallFunction|RearLights 1.0))))