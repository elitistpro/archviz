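; Interactable elevator that fakes travel by teleporting the player to a linked elevator.
; Overlapping its Open or Close trigger enables input, letting E toggle the doors through a DoOnce that resets when movement finishes.
; A timeline scrubs both elevator animations and resizes a box component alongside them.
; When the doors finish closing, the player moves to ElevatorToJump, which then opens.
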(event OnComponentBeginOverlap(Open)
  (params (OverlappedComponent :type Primitive%20Component%20Object%20Reference) (OtherActor :type Actor%20Object%20Reference) (OtherComp :type Primitive%20Component%20Object%20Reference) (OtherBodyIndex :type Integer) (bFromSweep :type Boolean) (SweepResult :type Hit%20Result%20Structure%20%28by%20ref%29))
  (Input|EnableInput (Game|GetPlayerController 0)))

(event OnComponentEndOverlap(Open)
  (params (OverlappedComponent :type Primitive%20Component%20Object%20Reference) (OtherActor :type Actor%20Object%20Reference) (OtherComp :type Primitive%20Component%20Object%20Reference) (OtherBodyIndex :type Integer))
  (Input|DisableInput (Game|GetPlayerController 0)))

(event OnComponentBeginOverlap(Close)
  (params (OverlappedComponent :type Primitive%20Component%20Object%20Reference) (OtherActor :type Actor%20Object%20Reference) (OtherComp :type Primitive%20Component%20Object%20Reference) (OtherBodyIndex :type Integer) (bFromSweep :type Boolean) (SweepResult :type Hit%20Result%20Structure%20%28by%20ref%29))
  (Input|EnableInput (Game|GetPlayerController 0)))

(event OnComponentEndOverlap(Close)
  (params (OverlappedComponent :type Primitive%20Component%20Object%20Reference) (OtherActor :type Actor%20Object%20Reference) (OtherComp :type Primitive%20Component%20Object%20Reference) (OtherBodyIndex :type Integer))
  (Input|DisableInput (Game|GetPlayerController 0)))

(event Custom|CloseElevator
  (bind _elevatortojump (Variables|Default|GetElevatorToJump))
  (bind _box4 (Variables|Default|GetBox4))
  (bind _boxextent (Variables|/Script/Engine.BoxComponent|GetBoxExtent _box4))
  (bind _value (Timeline|OpenCloseElevator ReverseFromEnd)
    (:Update
      (Components|Animation|SetPosition (Variables|Default|Getelevator_with_animation_lowpoly) (* _value 5.0) true)
      (Components|Box|SetBoxExtent _box4 (Math|Vector|MakeVector (- (.x _boxextent) (* _value 16.0)) (.y _boxextent) (.z _boxextent)) true))
    (:Finished
      (Utilities|FlowControl|Sequence
        (:then_0
          (Utilities|FlowControl|DoOnce false) ; enters at Reset
        )
        (:then_1
          (Variables|Default|SetOpenElevator%20? (> (* _value 5.0) 0.0))
          (Variables|Default|GetOpenElevator%20?
            (:then)
            (:else
              (Utilities|IsValid _elevatortojump
                (:Is%20Valid
                  (Transformation|SetActorLocation (Game|GetPlayerCharacter 0) (Math|Transform|TransformLocation (Transformation|GetActorTransform _elevatortojump) (Variables|BP_Elevator_C|GetActorLocation _elevatortojump)) false false)
                  (CallFunction|OpenElevator _elevatortojump))))))))))

(event Custom|OpenElevator
  (bind _elevatortojump (Variables|Default|GetElevatorToJump))
  (bind _box4 (Variables|Default|GetBox4))
  (bind _boxextent (Variables|/Script/Engine.BoxComponent|GetBoxExtent _box4))
  (bind _value (Timeline|OpenCloseElevator PlayFromStart)
    (:Update
      (Components|Animation|SetPosition (Variables|Default|Getelevator_with_animation_lowpoly) (* _value 5.0) true)
      (Components|Box|SetBoxExtent _box4 (Math|Vector|MakeVector (- (.x _boxextent) (* _value 16.0)) (.y _boxextent) (.z _boxextent)) true))
    (:Finished
      (Utilities|FlowControl|Sequence
        (:then_0
          (Utilities|FlowControl|DoOnce false) ; enters at Reset
        )
        (:then_1
          (Variables|Default|SetOpenElevator%20? (> (* _value 5.0) 0.0))
          (Variables|Default|GetOpenElevator%20?
            (:then)
            (:else
              (Utilities|IsValid _elevatortojump
                (:Is%20Valid
                  (Transformation|SetActorLocation (Game|GetPlayerCharacter 0) (Math|Transform|TransformLocation (Transformation|GetActorTransform _elevatortojump) (Variables|BP_Elevator_C|GetActorLocation _elevatortojump)) false false)
                  (CallFunction|OpenElevator _elevatortojump))))))))))

(event EventBeginPlay)

(event Collision|EventActorBeginOverlap
  (params (OtherActor :type Actor%20Object%20Reference)))

(event EventTick
  (params (DeltaSeconds :type Float%20%28single-precision%29)))

(event Input|KeyboardEvents|E
  (params (Key :type Key%20Structure :default "None"))
  (bind _elevatortojump (Variables|Default|GetElevatorToJump))
  (bind _box4 (Variables|Default|GetBox4))
  (bind _boxextent (Variables|/Script/Engine.BoxComponent|GetBoxExtent _box4))
  (:Pressed
    (Utilities|FlowControl|DoOnce false :!label _label
      (:Completed
        (Variables|Default|GetOpenElevator%20?
          (:then
            (bind _value (Timeline|OpenCloseElevator ReverseFromEnd)
              (:Update
                (Components|Animation|SetPosition (Variables|Default|Getelevator_with_animation_lowpoly) (* _value 5.0) true)
                (Components|Box|SetBoxExtent _box4 (Math|Vector|MakeVector (- (.x _boxextent) (* _value 16.0)) (.y _boxextent) (.z _boxextent)) true))
              (:Finished
                (Utilities|FlowControl|Sequence
                  (:then_0
                    (goto _label Reset))
                  (:then_1
                    (Variables|Default|SetOpenElevator%20? (> (* _value 5.0) 0.0))
                    (Variables|Default|GetOpenElevator%20?
                      (:then)
                      (:else
                        (Utilities|IsValid _elevatortojump
                          (:Is%20Valid
                            (Transformation|SetActorLocation (Game|GetPlayerCharacter 0) (Math|Transform|TransformLocation (Transformation|GetActorTransform _elevatortojump) (Variables|BP_Elevator_C|GetActorLocation _elevatortojump)) false false)
                            (CallFunction|OpenElevator _elevatortojump))))))))))
          (:else
            (Timeline|OpenCloseElevator PlayFromStart)))))))

(fn ConstructionScript)