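; 360 panorama sphere for the ArchViz explorer that switches between WC and RestRoom views via clickable arrow widgets.
; BeginPlay binds both WBP_360ArrowRoom widgets; each click applies a TexturesMap material by key, hides its own arrow and shows the other.
; The construction script creates a dynamic material, whose HDR_Texture BP_Explorer_PC changes through Update_360_Texture.
; Room switches replace that dynamic material on the sphere rather than updating its texture parameter.
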(event Custom|Update_360_Texture
  (params (360_Texture :type Texture%20Object%20Reference))
  ;[1 1 1] Change 360 Texture | Is called by BP_Explorer_PC
  (Rendering|Material|SetTextureParameterValue (Variables|Default|Get360_Dyn_Mat) "HDR_Texture" 360_Texture))

(event Custom|RestRoomClick
  (CallFunction|ApplyMaterialfromMap "RestRoom")
  (Rendering|SetVisibility (Variables|Default|GetArrowWCWidget) true false)
  (Rendering|SetVisibility (Variables|Default|GetRestRoomWidget) false false))

(event Custom|ArrowClick_Event
  (CallFunction|ApplyMaterialfromMap "WC")
  (Rendering|SetVisibility (Variables|Default|GetRestRoomWidget) true false)
  (Rendering|SetVisibility (Variables|Default|GetArrowWCWidget) false false))

(event EventBeginPlay
  (Utilities|FlowControl|Sequence
    (:then_0
      (bind _aswbp_360arrow_room (Utilities|Casting|CastToWBP_360ArrowRoom (UserInterface|GetWidget (Variables|Default|GetArrowWCWidget))))
      (Variables|Default|SetAs%20WBP%20360Arrow%20Room _aswbp_360arrow_room)
      (EventDispatchers|AssignArrowClick (Variables|Default|GetAs%20WBP%20360Arrow%20Room) (delegate Custom|ArrowClick_Event)))
    (:then_1
      (bind _aswbp_360arrow_room_2 (Utilities|Casting|CastToWBP_360ArrowRoom (UserInterface|GetWidget (Variables|Default|GetRestRoomWidget))))
      (EventDispatchers|AssignArrowClick _aswbp_360arrow_room_2 (delegate Custom|RestRoomClick)))))

(fn ConstructionScript
  (bind _sphere (Variables|Default|GetSphere))
  ;[1 1 1] Create Dynamic Sphere Material - This allows to change the texture during play
  (bind _returnvalue (Rendering|Material|CreateDynamicMaterialInstance _sphere 0 (Rendering|Material|GetMaterial _sphere 0) "" :!class /Script/Engine.PrimitiveComponent))
  (bind _output_get (Variables|Default|Set360_Dyn_Mat _returnvalue))
  (Rendering|Material|SetMaterial (Variables|Default|GetSphere) 0 _output_get))

(fn ApplyMaterialfromMap
  (params (ItemToFind :type String))
  (bind _texturesmap (Variables|Default|GetTexturesMap))
  (bind _keys (Utilities|Map|Keys _texturesmap))
  (Rendering|Material|SetMaterial (Variables|Default|GetSphere) 0 (.Value (Utilities|Map|GetKeyValueByIndex _texturesmap (Utilities|Array|FindItem _keys ItemToFind)))))