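; Game instance for ArchViz Explorer that holds the save data manager and tracks Points of Interest (POI) across the app.
; On Init it creates a DataManager save object, keeps it as SaveDataManager and loads it.
; Store_Current_Visibility rebuilds BPPOIsVisible from the POIs in BPPOIs flagged as Showing.
; Disconnected leftover nodes check for a save and copy POI data table rows into the save manager.
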(event Custom|Store_Current_Visibility
  (Utilities|Array|Clear (Variables|Default|GetBP_POIs_Visible))
  (for _array_element (Variables|Default|GetBP_POIs)
    (if (Variables|/Game/ArchVizExplorer/Blueprints/BP_POI.BP_POI_C|GetShowing? _array_element)
      (Utilities|Array|AddUnique (Variables|Default|GetBP_POIs_Visible) _array_element))))

(event EventInit
  (bind _returnvalue (SaveGame|CreateSaveGameObject "/Game/Blueprints/DataManager.DataManager_C"))
  (bind _output_get (Variables|Default|SetSaveDataManager _returnvalue))
  (Default|Load _output_get))