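; DataManager is a save game object that stores point-of-interest structs in a SaveData map keyed by name.
; Add and Edit both write entries to the map; Find and FindPure read them, with Find also printing the entry's Availability.
; Save writes the object itself to its slot, and Load copies the map back from the saved copy.
; Delete and GetAll are empty stubs.
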(fn Add
  (params (Name :type Text) (POI%20Struct :type POI%20Filter%20Struct%20Structure))
  (Utilities|Map|Add (Variables|Default|GetSaveData) (Utilities|String|ToString(Text) Name) POI%20Struct))

(fn Edit
  (params (Name :type Name) (POI%20Filter :type POI%20Filter%20Struct%20Structure))
  (Utilities|Map|Add (Variables|Default|GetSaveData) (Utilities|String|ToString(Name) Name) POI%20Filter))

(fn Delete)

(fn Find
  (params (Name :type Name))
  (bind _returnvalue (Utilities|String|ToString(Name) Name))
  (bind _savedata (Variables|Default|GetSaveData))
  (bind _value (Utilities|Map|Find _savedata _returnvalue))
  (Development|PrintString 0 (Utilities|String|EnumtoString (.Availability (Utilities|Struct|BreakPOI_Filter_Struct _value))))
  (return _value))

(fn GetAll)

(fn Save
  (SaveGame|SaveGametoSlot self (Variables|Default|GetSaveSlotName)))

(fn Load
  (bind _returnvalue (SaveGame|LoadGamefromSlot (Variables|Default|GetSaveSlotName)))
  (bind _asdata_manager (Utilities|Casting|CastToDataManager _returnvalue))
  (Variables|Default|SetSaveData (Variables|DataManager_C|GetSaveData _asdata_manager)))

(fn FindPure
  (params (Name :type Name))
  (return (.Value (Utilities|Map|Find (Variables|Default|GetSaveData) (Utilities|String|ToString(Name) Name)))))